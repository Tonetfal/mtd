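; Base tower pawn that automatically fires projectiles at targets chosen by its BP_TowerController.
; On BeginPlay it passes vision range and angle to the controller, then polls it for a fire target each Tick while not reloading.
; OnFire spawns the projectile class, configures it as homing or directional with optional radial damage, and starts a reload timer.
; "Scaled" getters define stat hooks based on the base values, with reload time derived from fire rate.
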(event EventBeginPlay
  (bind _asbp_tower_controller (Utilities|Casting|CastToBP_TowerController (Pawn|GetController)))
  (Class|MTDTowerController|SetVisionRange _asbp_tower_controller (Variables|MTD|Fire|GetBaseVisionRange))
  (Class|MTDTowerController|SetPeripheralVisionHalfAngleDegrees _asbp_tower_controller (Variables|MTD|Fire|GetBaseVisionHalfDegrees)))

(event EventTick
  (params (DeltaSeconds :type Float%20%28single-precision%29))
  (if (not (Variables|MTD|Fire|GetbIsReloading))
    (bind _asbp_tower_controller (Utilities|Casting|CastToBP_TowerController (Pawn|GetController)))
    (bind _returnvalue (Class|MTDTowerController|GetFireTarget _asbp_tower_controller))
    (CallFunction|OnFire _returnvalue)))

(fn ConstructionScript)

(fn OnFire
  (params (Fire%20Target :type Actor%20Object%20Reference))
  (bind _speed (Utilities|GetScaledProjectileSpeed))
  (bind _speed_2 (Utilities|GetScaledProjectileSpeed))
  (bind _output_get (LocalVariables|SetFireTarget Fire%20Target))
  (Utilities|IsValid _output_get
    (:Is%20Valid
      (if (Utilities|IsValidClass (Variables|MTD|Projectile|GetProjectileClass))
        (LocalVariables|SetDirectionTowardsTarget (/ (- (Transformation|GetActorLocation (LocalVariables|GetFireTarget)) (Transformation|GetWorldLocation (Variables|MTD|Components|GetProjectileSpawnPosition))) (Math|Vector|VectorLength (- (Transformation|GetActorLocation (LocalVariables|GetFireTarget)) (Transformation|GetWorldLocation (Variables|MTD|Components|GetProjectileSpawnPosition))))))
        (bind _returnvalue (Game|SpawnActorfromClass (Variables|MTD|Projectile|GetProjectileClass) (Math|Transform|MakeTransform (Transformation|GetWorldLocation (Variables|MTD|Components|GetProjectileSpawnPosition)) (Transformation|GetActorRotation)) "AlwaysSpawn" self 0))
        (LocalVariables|SetProjectile _returnvalue)
        (if (Variables|MTD|Projectile|GetbAreProjectilesHoming)
          (Class|MTDProjectile|SetupParameters (LocalVariables|GetProjectile) (Utilities|Struct|MakeMTD_ProjectileParameters _speed _speed _speed (Utilities|GetScaledDamage) (Variables|MTD|Projectile|GetbAreProjectilesRadial) (Variables|MTD|Projectile|GetBaseProjectileExplosionRadius) false (LocalVariables|GetFireTarget) "0.000000,0.000000,0.000000" (.name (Variables|MTD|Projectile|GetProjectileCollisionProfileName))))
          (else
            (Class|MTDProjectile|SetupParameters (LocalVariables|GetProjectile) (Utilities|Struct|MakeMTD_ProjectileParameters _speed_2 _speed_2 _speed_2 (Utilities|GetScaledDamage) (Variables|MTD|Projectile|GetbAreProjectilesRadial) (Variables|MTD|Projectile|GetBaseProjectileExplosionRadius) false 0 (LocalVariables|GetDirectionTowardsTarget) (.name (Variables|MTD|Projectile|GetProjectileCollisionProfileName))))))
        (Variables|MTD|Fire|SetbIsReloading true)
        (bind _returnvalue_2 (Utilities|Time|SetTimerbyFunctionName 0 "OnReloadFinished" (Utilities|GetReloadTime)))
        (Variables|MTD|Fire|SetReloadTimerHandle _returnvalue_2)))))

(fn OnReloadFinished
  (Variables|MTD|Fire|SetbIsReloading false))