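; Base player character Blueprint for heroes, translating axis input into actor-relative movement and controller yaw and pitch.
; Turn input also records a turning flag and ratio, which ConsumeTurnRatio returns and clears in one read.
; OnReset enables controller-desired rotation, while DisableControllerInput turns it off and, despite its name, sets ignore-move-input to false.
; The OnJumped event calls Jump.
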(event EventBeginPlay
  (|CallParentFunction) ; This node is disabled and will not be called.\nDrag off pins to build functionality.
)

(event Collision|EventActorBeginOverlap
  (params (OtherActor :type Actor%20Object%20Reference)))

(event EventTick
  (params (DeltaSeconds :type Float%20%28single-precision%29))
  (|CallParentFunction DeltaSeconds) ; This node is disabled and will not be called.\nDrag off pins to build functionality.
)

(event EventOnReset
  (Variables|/Script/Engine.CharacterMovementComponent|SetbUseControllerDesiredRotation (Variables|Character|GetCharacterMovement) true))

(event EventOnJumped
  (Character|Jump))

(event Input|AxisEvents|InputAxisTurnRight
  (params (AxisValue :type Float%20%28single-precision%29))
  (Variables|MTD|Animation|SetbIsTurning true)
  (Variables|MTD|Animation|SetTurnRatio AxisValue)
  (Pawn|Input|AddControllerYawInput AxisValue))

(event Input|AxisEvents|InputAxisLookUp
  (params (AxisValue :type Float%20%28single-precision%29))
  (Pawn|Input|AddControllerPitchInput AxisValue))

(event Input|AxisEvents|InputAxisMoveForward
  (params (AxisValue :type Float%20%28single-precision%29))
  (Pawn|Input|AddMovementInput (Transformation|GetActorForwardVector) AxisValue false))

(event Input|AxisEvents|InputAxisMoveRight
  (params (AxisValue :type Float%20%28single-precision%29))
  (Pawn|Input|AddMovementInput (Transformation|GetActorRightVector) AxisValue false))

(fn ConstructionScript
  (|CallParentFunction))

(fn ConsumeTurnRatio
  (LocalVariables|SetTurnRatioTmp (Variables|MTD|Animation|GetTurnRatio))
  (LocalVariables|SetbIsTurningTmp (Variables|MTD|Animation|GetbIsTurning))
  (Variables|MTD|Animation|SetbIsTurning false)
  (Variables|MTD|Animation|SetTurnRatio 0.0)
  (return (LocalVariables|GetbIsTurningTmp) (LocalVariables|GetTurnRatioTmp)))

(fn DisableControllerInput
  (bind _returnvalue (Pawn|GetController))
  (bind _charactermovement (Variables|Character|GetCharacterMovement))
  (Utilities|IsValid _returnvalue
    (:Is%20Valid
      (Input|SetIgnoreMoveInput _returnvalue false)
      (Utilities|IsValid _charactermovement
        (:Is%20Valid
          (Variables|/Script/Engine.CharacterMovementComponent|SetbUseControllerDesiredRotation _charactermovement false))))))