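; Base character Blueprint that grants GAS abilities through the player state and handles melee hit detection and death.
; It maps hitbox data by nickname, and events add or remove active hitboxes.
; While any are active, Tick sphere-traces them, sending itself a gameplay event per new target until reset.
; HealthComponent death events stop movement and collision, then destroy the actor; a helper computes signed movement angle.
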(event EventBeginPlay
  (bind _healthcomponent (Variables|Default|GetHealthComponent))
  (CallFunction|ContructHitboxMap)
  (CallFunction|InitializeAbilities)
  (EventDispatchers|AssignOnDeathStarted _healthcomponent (EventDispatchers|CreateEvent :!event EventonDeathStarted))
  (EventDispatchers|AssignOnDeathFinished _healthcomponent (EventDispatchers|CreateEvent :!event EventonDeathFinished)))

(event EventTick
  (params (DeltaSeconds :type Float%20%28single-precision%29))
  (if (Variables|MTD|Attack|GetIsMeleeInProgress)
    (CallFunction|EventPerformHitboxTrace)))

(event Custom|CancelAttackMelee
  (CallFunction|DisableMeleeHitboxes))

(event Custom|EventPerformHitboxTrace
  (bind _meleehittargets (Variables|MTD|Attack|GetMeleeHitTargets))
  (if (> (Utilities|Array|Length (Variables|MTD|Attack|GetActiveHitboxes)) 0)
    (for _array_element (Variables|MTD|Attack|GetActiveHitboxes)
      (bind (_outhits _returnvalue) (Collision|MultiSphereTraceForObjects (+ (Transformation|GetActorLocation) (Math|Vector|RotateVector (.Offset (Utilities|Struct|BreakMeleeHitSphereDefinition _array_element)) (Math|Conversions|RotationFromXVector (Transformation|GetActorForwardVector)))) (+ (Transformation|GetActorLocation) (Math|Vector|RotateVector (.Offset (Utilities|Struct|BreakMeleeHitSphereDefinition _array_element)) (Math|Conversions|RotationFromXVector (Transformation|GetActorForwardVector)))) (.Radius (Utilities|Struct|BreakMeleeHitSphereDefinition _array_element)) (Variables|MTD|Attack|GetTargetCollisionProfilesToHit) false 0 (select (Variables|MTD|Attack|GetDebugMelee) "ForDuration" "None") true "(R=1.000000,G=0.000000,B=0.000000,A=1.000000)" "(R=0.000000,G=1.000000,B=0.000000,A=1.000000)" 0.0))
      (if _returnvalue
        (for _array_element_2 _outhits
          (if (not (Utilities|Array|ContainsItem _meleehittargets (.HitActor (Collision|BreakHitResult _array_element_2))))
            (Utilities|Array|AddUnique _meleehittargets (.HitActor (Collision|BreakHitResult _array_element_2)))
            (Ability|SendGameplayEventtoActor self "(TagName=\"GameplayCue.AttackMelee\")" (Utilities|Struct|MakeGameplayEventData "(TagName=\"Ability.Attack.Melee\")" self (.HitActor (Collision|BreakHitResult _array_element_2)) 0 0 (GameplayEffects|MakeEffectContext (Class|MTDBaseCharacter|GetMtdAbilitySystemComponent)) "(GameplayTags=)" "(GameplayTags=)" 1.0 (Ability|TargetData|AbilityTargetDatafromHitResult _array_element_2)))))))))

(event EventAddMeleeHitboxes
  (params (MeleeHitboxes :type Array%20of%20Names))
  ;[1 1 1] Adds hitboxes with the given nicknames.
  (for _array_element MeleeHitboxes
    (if (.ReturnValue (Utilities|Map|Find (Variables|MTD|Attack|GetHitboxMap) _array_element))
      (Utilities|Array|AddUnique (Variables|MTD|Attack|GetActiveHitboxes) (Utilities|Struct|BreakActiveHitboxEntry (.Value (Utilities|Map|Find (Variables|MTD|Attack|GetHitboxMap) _array_element))))))
  (Variables|MTD|Attack|SetIsMeleeInProgress (> (Utilities|Array|Length (Variables|MTD|Attack|GetActiveHitboxes)) 0)))

(event EventDisableMeleeHitboxes
  ;[1 1 1] Forcibly kills all active melee hitboxes, and empties the list.
  (Variables|MTD|Attack|SetIsMeleeInProgress false)
  (Utilities|Array|Clear (Variables|MTD|Attack|GetActiveHitboxes))
  (CallFunction|ResetMeleeHitboxes))

(event EventResetMeleeHitboxes
  ;[1 1 1] Resets the active hitboxes so that hit detection can be performed on target again.
  (Utilities|Array|Clear (Variables|MTD|Attack|GetMeleeHitTargets)))

(event EventRemoveMeleeHitboxes
  (params (MeleeHitboxes :type Array%20of%20Names))
  ;[1 1 1] Removes hitboxes with the given nicknames.
  (for _array_element MeleeHitboxes
    (if (.ReturnValue (Utilities|Map|Find (Variables|MTD|Attack|GetHitboxMap) _array_element))
      (Utilities|Array|RemoveItem (Variables|MTD|Attack|GetActiveHitboxes) (Utilities|Struct|BreakActiveHitboxEntry (.Value (Utilities|Map|Find (Variables|MTD|Attack|GetHitboxMap) _array_element))))))
  (Variables|MTD|Attack|SetIsMeleeInProgress (> (Utilities|Array|Length (Variables|MTD|Attack|GetActiveHitboxes)) 0)))

(fn ConstructionScript)

(fn InitializeAbilities
  (bind _returnvalue (Class|MTDBaseCharacter|GetMtdPlayerState))
  (Utilities|IsValid _returnvalue
    (:Is%20Valid
      (for (_array_element _array_index) (Variables|MTD|AbilitySystem|GetAbilityList)
        (Class|MTDPlayerState|GrantAbility _returnvalue _array_element 1 _array_index)))
    (:Is%20Not%20Valid
      (Development|PrintString "BP_MtdPlayerCharacter has an invalid MTD_PlayerState" true true "(R=1.000000,G=0.000000,B=0.027873,A=1.000000)" 1e+01))))

(fn ContructHitboxMap
  (Utilities|Map|Clear (Variables|MTD|Attack|GetHitboxMap))
  (for _array_element (Variables|/Script/mtd.MeleeHitboxData|GetMeleeHitSpheres (Variables|MTD|Attack|GetHitboxData))
    (Utilities|Map|Add (Variables|MTD|Attack|GetHitboxMap) (.Nickname (Utilities|Struct|BreakMeleeHitSphereDefinition _array_element)) (Utilities|Struct|MakeActiveHitboxEntry _array_element))))

(fn EventonDeathStarted
  (params (OwningActor :type Actor%20Object%20Reference))
  (Utilities|FlowControl|Sequence
    (:then_0
      (CallFunction|DisableControllerInput))
    (:then_1
      (CallFunction|DisableMovement))
    (:then_2
      (CallFunction|DIsableCollision))))

(fn EventonDeathFinished
  (params (OwningActor :type Actor%20Object%20Reference))
  (Actor|DestroyActor))

(fn DisableControllerInput
  (bind _returnvalue (Pawn|GetController))
  (Utilities|IsValid _returnvalue
    (:Is%20Valid
      (Input|SetIgnoreMoveInput _returnvalue false)
      (Input|SetIgnoreLookInput _returnvalue false))))

(fn DisableMovement
  (bind _charactermovement (Variables|Character|GetCharacterMovement))
  (Utilities|IsValid _charactermovement
    (:Is%20Valid
      (Components|Movement|StopMovementImmediately _charactermovement)
      (Pawn|Components|CharacterMovement|DisableMovement _charactermovement))))

(fn DIsableCollision
  (bind _capsulecomponent (Variables|Default|GetCapsuleComponent))
  (Utilities|IsValid _capsulecomponent
    (:Is%20Valid
      (Collision|SetCollisionEnabled _capsulecomponent "NoCollision")
      (Collision|SetCollisionResponsetoAllChannels _capsulecomponent "ECR_Ignore"))))

(fn GetMovementDirectionAngle
  (bind _returnvalue (Transformation|GetVelocity))
  (bind _returnvalue_2 (Transformation|GetActorForwardVector))
  (bind _returnvalue_3 (Class|KismetMathLibrary|VectorNormalUnsafe _returnvalue))
  (bind _returnvalue_4 (Math|Vector|DotProduct _returnvalue_2 _returnvalue_3))
  (bind _returnvalue_5 (Math|Vector|CrossProduct _returnvalue_2 _returnvalue_3))
  (bind _returnvalue_6 (Class|KismetMathLibrary|DegAcos _returnvalue_4))
  (if (not (Math|Vector|VectorIsZero _returnvalue))
    (if (Math|Vector|VectorIsZero _returnvalue_5)
      (return _returnvalue_6)
      (else
        (return (* _returnvalue_6 (Math|Float|Sign(Float) (.Z (Class|KismetMathLibrary|BreakVector3f _returnvalue_5)))))))))