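; Base enemy Blueprint that handles attack target selection and removal after death.
; Two spheres maintain detected targets; Tick uses line traces to drop unseen targets and pick visible ones, unless targeting is temporarily forced.
; Target changes rebind death listeners and notify a dispatcher, while unreachable targets are ignored until a successful path arrival or a lose-sight overlap ends.
; Timers delay destruction after death and gradually shrink the actor before destroying it.
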(event OnComponentBeginOverlap(SightSphere)
  (params (OverlappedComponent :type Primitive%20Component%20Object%20Reference) (OtherActor :type Actor%20Object%20Reference) (OtherComp :type Primitive%20Component%20Object%20Reference) (OtherBodyIndex :type Integer) (bFromSweep :type Boolean) (SweepResult :type Hit%20Result%20Structure%20%28by%20ref%29))
  (if (!= OtherActor (Variables|MTD|Attack|GetIgnoredActor))
    (Utilities|Array|Add (Variables|MTD|Attack|GetDetectedTargets) OtherActor)))

(event OnComponentEndOverlap(LoseSightSphere)
  (params (OverlappedComponent :type Primitive%20Component%20Object%20Reference) (OtherActor :type Actor%20Object%20Reference) (OtherComp :type Primitive%20Component%20Object%20Reference) (OtherBodyIndex :type Integer))
  (Utilities|Array|RemoveItem (Variables|MTD|Attack|GetDetectedTargets) 0)
  (CallFunction|OnIgnoreActorClear)
  (if (== OtherActor (Variables|MTD|Attack|GetAttackTarget))
    (CallFunction|ClearAttackTarget)))

(event Custom|ScaleDown
  (Transformation|SetActorRelativeScale3D (- (Transformation|GetActorScale3D) (* (/ (/ 1.0 (Variables|MTD|Death|GetScaleDownTicksPerSecond)) (Variables|MTD|Death|GetSecondsToCompleteScaleDown)) (Variables|MTD|Death|GetInitialScale)))))

(event Custom|OnDestroy
  (Variables|MTD|Death|SetInitialScale (Transformation|GetActorScale3D))
  (bind _returnvalue (Utilities|Time|SetTimerbyEvent (delegate Custom|ScaleDown) (/ 1.0 (Variables|MTD|Death|GetScaleDownTicksPerSecond)) true))
  (Utilities|Time|SetTimerbyEvent (delegate Custom|FinishScalingDown) (Variables|MTD|Death|GetSecondsToCompleteScaleDown)))

(event Custom|EventOnDestinationDelegate
  (params (bSuccess :type Boolean))
  (if bSuccess
    (CallFunction|OnIgnoreActorClear)))

(event Custom|FinishScalingDown
  (Utilities|Time|ClearandInvalidateTimerbyHandle (stale Custom|OnDestroy _returnvalue))
  (Actor|DestroyActor))

(event EventBeginPlay
  (EventDispatchers|AssignOnDestinationDelegate (Variables|Default|GetMTD%20Path%20Following) (delegate Custom|EventOnDestinationDelegate))
  (EventDispatchers|AssignOnDeathFinished (Variables|Default|GetHealthComponent) (EventDispatchers|CreateEvent :!event OnDeath)))

(event EventTick
  (params (DeltaSeconds :type Float%20%28single-precision%29))
  (if (not (Variables|MTD|Attack|GetbForceTarget))
    (Utilities|IsValid (Variables|MTD|Attack|GetAttackTarget)
      (:Is%20Valid
        (bind _return_value (CallFunction|CanbeSeen (Variables|MTD|Attack|GetAttackTarget)))
        (if (not _return_value)
          (CallFunction|ClearAttackTarget)
          (CallFunction|CleanInvalidTargets :!label _label)
          (bind _array_element (Utilities|Array|ForEachLoopwithBreak (Variables|MTD|Attack|GetDetectedTargets) :!label _label_2)
            (:LoopBody
              (bind _return_value_2 (CallFunction|CanbeSeen _array_element))
              (if _return_value_2
                (CallFunction|SetNewAttackTarget _array_element false)
                (goto _label_2 Break))))))
      (:Is%20Not%20Valid
        (goto _label)))))

(fn ConstructionScript
  (|CallParentFunction))

(fn OnStartForceTargetting
  (params (Duration :type Float%20%28double-precision%29))
  (Variables|MTD|Attack|SetbForceTarget true)
  (bind _returnvalue (Utilities|Time|SetTimerbyFunctionName 0 "OnStopForceTargetting" Duration))
  (Variables|MTD|Attack|SetStopForceTargettingTimerHandle _returnvalue))

(fn OnStopForceTargetting
  (Variables|MTD|Attack|SetbForceTarget false))

(fn SetNewAttackTarget
  (params (NewTarget :type Actor%20Object%20Reference) (ForceTarget :type Boolean))
  (bind _returnvalue (Actor|GetComponentbyClass "/Script/mtd.MTD_HealthComponent"))
  (if (!= NewTarget (Variables|MTD|Attack|GetAttackTarget))
    (Utilities|FlowControl|Sequence
      (:then_0
        (Utilities|FlowControl|Sequence
          (:then_0
            (Utilities|IsValid (Variables|MTD|Attack|GetAttackTarget)
              (:Is%20Valid
                (Utilities|IsValid (Actor|GetComponentbyClass (Variables|MTD|Attack|GetAttackTarget) "/Script/mtd.MTD_HealthComponent")
                  (:Is%20Valid
                    (EventDispatchers|UnbindEventfromOnDeathStarted (Actor|GetComponentbyClass (Variables|MTD|Attack|GetAttackTarget) "/Script/mtd.MTD_HealthComponent") (EventDispatchers|CreateEvent :!event OnAttackTargetDied)))))))
          (:then_1
            (Utilities|IsValid NewTarget
              (:Is%20Valid
                (Utilities|IsValid _returnvalue
                  (:Is%20Valid
                    (EventDispatchers|BindEventtoOnDeathStarted _returnvalue (EventDispatchers|CreateEvent :!event OnAttackTargetDied)))))))
          (:then_2
            (Default|CallNewTargetEventDispatcher (Variables|MTD|Attack|GetAttackTarget) NewTarget)
            (Variables|MTD|Attack|SetAttackTarget NewTarget))))
      (:then_1
        (if ForceTarget
          (CallFunction|OnStartForceTargetting (Variables|MTD|Attack|GetForceTargetDuration)))))))

(fn OnDeathFinished1)

(fn OnAttackTargetDied
  (params (OwningActor :type Actor%20Object%20Reference))
  (Variables|MTD|Attack|SetAttackTarget 0)
  (Variables|MTD|Attack|SetbForceTarget false)
  (Utilities|Time|ClearandInvalidateTimerbyHandle (Variables|MTD|Attack|GetStopForceTargettingTimerHandle))
  (CallFunction|OnStopForceTargetting))

(fn CleanInvalidTargets
  (bind _detectedtargets (Variables|MTD|Attack|GetDetectedTargets))
  (for _array_element _detectedtargets
    (Utilities|IsValid _array_element
      (:Is%20Not%20Valid
        (Utilities|Array|RemoveItem _detectedtargets _array_element)))))

(fn CanbeSeen
  (params (Target :type Actor%20Object%20Reference))
  (bind _returnvalue (Transformation|GetActorLocation))
  (bind _returnvalue_2 (Transformation|GetActorLocation))
  (bind _returnvalue_3 (Transformation|GetActorLocation Target))
  (bind _returnvalue_4 (- _returnvalue_3 _returnvalue))
  (bind _outhit (Collision|LineTraceByChannel _returnvalue_2 (+ _returnvalue_2 (* (/ _returnvalue_4 (Math|Vector|VectorLength _returnvalue_4)) (Components|Sphere|GetScaledSphereRadius (Variables|Default|GetLoseSightSphere)))) "TraceTypeQuery3" false 0 "None"))
  (return (== Target (.HitActor (Collision|BreakHitResult _outhit)))))

(fn OnTargetNonReacheable
  (CallFunction|OnAttackTargetIgnore true))

(fn OnAttackTargetIgnore
  (params (OverrideAttackTarget :type Boolean))
  (bind _attacktarget (Variables|MTD|Attack|GetAttackTarget))
  (Utilities|FlowControl|Sequence
    (:then_0
      (Utilities|Array|RemoveItem (Variables|MTD|Attack|GetDetectedTargets) _attacktarget)
      (Variables|MTD|Attack|SetIgnoredActor _attacktarget))
    (:then_1
      (if OverrideAttackTarget
        (CallFunction|ClearAttackTarget)))))

(fn OnIgnoreActorClear
  (Variables|MTD|Attack|SetIgnoredActor 0))

(fn ClearAttackTarget
  (CallFunction|SetNewAttackTarget 0 false))

(fn OnDeath
  (params (OwningActor :type Actor%20Object%20Reference))
  (Utilities|Time|SetTimerbyEvent (EventDispatchers|CreateEvent :!event Custom|OnDestroy) (Variables|MTD|Death|GetSecondsToStartDestroying)))