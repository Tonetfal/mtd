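; Melee enemy Blueprint that adds a delayed shrink-and-remove sequence on death.
; After calling the parent OnDeath, it waits on a timer, then records the actor's scale.
; A looping timer subtracts a fixed fraction of that scale each step, giving a linear shrink without using Tick.
; A second timer ends the loop and destroys both the held weapon and the enemy.
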(event Custom|ScaleDown
  (Transformation|SetActorRelativeScale3D (- (Transformation|GetActorScale3D) (* (/ (/ 1.0 (Variables|Default|GetScaleDownTicksPerSecond)) (Variables|Default|GetSecondsToCompleteScaleDown)) (Variables|Default|GetInitialScale)))))

(event Custom|OnDestroy
  (Variables|Default|SetInitialScale (Transformation|GetActorScale3D))
  (bind _returnvalue (Utilities|Time|SetTimerbyEvent (delegate Custom|ScaleDown) (/ 1.0 (Variables|Default|GetScaleDownTicksPerSecond)) true))
  (Utilities|Time|SetTimerbyEvent (delegate Custom|FinishScalingDown) (Variables|Default|GetSecondsToCompleteScaleDown)))

(event Custom|FinishScalingDown
  (Utilities|Time|ClearandInvalidateTimerbyHandle (stale Custom|OnDestroy _returnvalue))
  (Actor|DestroyActor (Variables|/Script/mtd.MTD_WeaponComponent|GetWeapon (Variables|Default|GetWeapon)))
  (Actor|DestroyActor))

(event EventBeginPlay)

(event Collision|EventActorBeginOverlap
  (params (OtherActor :type Actor%20Object%20Reference)))

(event EventTick
  (params (DeltaSeconds :type Float%20%28single-precision%29)))

(event EventOnDeath
  (|CallParentFunction)
  (Utilities|Time|SetTimerbyEvent (delegate Custom|OnDestroy) (Variables|Default|GetSecondsToStartDestroying)))

(fn ConstructionScript)