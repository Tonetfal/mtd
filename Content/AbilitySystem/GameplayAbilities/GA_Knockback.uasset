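; GA_Knockback is an event-triggered gameplay ability that knocks its avatar character back after a balance hit.
; It reads balance hit data from the event's second optional object, then launches the character along the horizontal knockback direction, scaled by balance damage and a per-damage travel factor.
; It plays a random ability montage and ends immediately without waiting for it, printing an error if either cast fails.
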(event Ability|EventActivateAbility
  (|CallParentFunction)
  (bind _asmtd_balance_hit_data (Utilities|Casting|CastToMTD_BalanceHitData (.OptionalObject2 (Utilities|Struct|BreakGameplayEventData (Variables|Default|GetGameplayEventData))))
    (:then
      (Variables|Default|SetHitData _asmtd_balance_hit_data)
      (bind _ascharacter (Utilities|Casting|CastToCharacter (Ability|GetAvatarActorfromActorInfo))
        (:then
          (Variables|Default|SetCharacter _ascharacter)
          (Utilities|FlowControl|Sequence
            (:then_0
              (Character|LaunchCharacter (Variables|Default|GetCharacter) (* (Class|KismetMathLibrary|VectorNormal2D (Variables|/Script/mtd.MTD_BalanceHitData|GetKnockbackDirection (Variables|Default|GetHitData)) 0.0001) (* (Variables|/Script/mtd.MTD_BalanceHitData|GetBalanceDamage (Variables|Default|GetHitData)) (Variables|Default|GetUnitsToTravelOnBalanceDamageOfOne))) false true))
            (:then_1
              (Animation|PlayAnimMontage (Variables|Default|GetCharacter) (Class|MTDGameplayAbility|GetRandomAbilityAnimMontage) 1.0 "None"))
            (:then_2
              (Ability|EndAbility))))
        (:CastFailed
          (Development|PrintString "Failed to cast Avatar Actor to Character.")
          (Ability|EndAbility :!label _label))))
    (:CastFailed
      (Development|PrintString "Failed to cast Optional Object 2 to Balance Hit Data.")
      (goto _label))))