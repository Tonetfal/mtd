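; Gameplay ability that starts a wave in the tower defense game mode.
; Activation gets the WaveManager from BP_TowerDefenseMode, calls StartWave on it, then ends the ability.
; CanActivateAbility allows activation only when the current game mode is a BP_TowerDefenseMode.
; If the cast fails or WaveManager is invalid, activation does not reach EndAbility.
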(event Ability|EventActivateAbility
  (|CallParentFunction)
  (bind _asbp_tower_defense_mode (Utilities|Casting|CastToBP_TowerDefenseMode (Game|GetGameMode)))
  (Utilities|IsValid (Variables|/Script/mtd.MTD_TowerDefenseMode|GetWaveManager _asbp_tower_defense_mode)
    (:Is%20Valid
      (Class|MTDWaveManager|StartWave (Variables|/Script/mtd.MTD_TowerDefenseMode|GetWaveManager _asbp_tower_defense_mode))
      (Ability|EndAbility))))

(event Ability|EventOnEndAbility
  (params (bWasCancelled :type Boolean))
  (|CallParentFunction bWasCancelled) ; This node is disabled and will not be called.\nDrag off pins to build functionality.
)

(fn K2CanActivateAbility
  (params (ActorInfo :type Gameplay%20Ability%20Actor%20Info%20Structure) (Handle :type Gameplay%20Ability%20Spec%20Handle%20Structure))
  (bind _returnvalue (Game|GetGameMode))
  (Utilities|IsValid _returnvalue
    (:Is%20Valid
      (Utilities|Casting|CastToBP_TowerDefenseMode _returnvalue
        (:then
          (return "" true))
        (:CastFailed
          (return "" false))))))