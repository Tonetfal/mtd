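; Base gameplay ability Blueprint that supplies helpers for building outgoing damage effect specs.
; Two functions pass either the instant or the ranged instant damage GameplayEffect class to a shared implementation.
; That implementation validates the ability system component and effect class, makes a level 1 spec, and writes the ability's additive and multiplier damage values as SetByCaller magnitudes.
; Activate and end events are unused stubs.
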(event Ability|EventActivateAbility)

(event Ability|EventOnEndAbility
  (params (bWasCancelled :type Boolean)))

(fn CreateOutgoingDamageSpecHandle
  (return (CallFunction|CreateOutgoingDamageSpecHandleImplementation "/Game/AbilitySystem/Effects/GE_DamageInstant.GE_DamageInstant_C")))

(fn CreateOutgoingRangedDamageSpecHandle
  (return (CallFunction|CreateOutgoingDamageSpecHandleImplementation "/Game/AbilitySystem/Effects/GE_RangedDamageInstant.GE_RangedDamageInstant_C")))

(fn CreateOutgoingDamageSpecHandleImplementation
  (params (GeDamageClass :type Gameplay%20Effect%20Class%20Reference))
  (bind _returnvalue (Ability|GetAbilitySystemComponentfromActorInfo))
  (Utilities|IsValid _returnvalue
    (:Is%20Valid
      (if (Utilities|IsValidClass GeDamageClass)
        (bind _returnvalue_2 (Ability|GameplayEffect|AssignTagSetbyCallerMagnitude (GameplayEffects|MakeOutgoingSpec _returnvalue GeDamageClass 1.0 (GameplayEffects|MakeEffectContext _returnvalue)) "(TagName=\"SetByCaller.Damage.Additive\")" (Variables|Default|GetDamageAdditive)))
        (bind _returnvalue_3 (Ability|GameplayEffect|AssignTagSetbyCallerMagnitude _returnvalue_2 "(TagName=\"SetByCaller.Damage.Multiplier\")" (Variables|Default|GetDamageMultiplier)))
        (return _returnvalue_3)
        (else
          _)))
    (:Is%20Not%20Valid
      _))
  (return ""))