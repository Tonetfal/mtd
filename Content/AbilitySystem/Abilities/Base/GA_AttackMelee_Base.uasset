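; Base melee attack gameplay ability that applies instant damage to the targets of a strike.
; On activation it waits for the Animation.MeleeStrike gameplay event, whose payload carries the target data.
; Each event builds a GE_DamageInstant spec, sets additive and multiplier damage through SetByCaller tags from the ability's variables, and applies it to those targets.
; The graph itself plays no montage and never commits or ends the ability.
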(event Ability|EventActivateAbility
  (bind _returnvalue (Ability|GetAbilitySystemComponentfromActorInfo))
  (bind _payload (Ability|Tasks|WaitGameplayEvent "(TagName=\"Animation.MeleeStrike\")" 0)
    (:EventReceived
      (bind _returnvalue_2 (Ability|GameplayEffect|AssignTagSetbyCallerMagnitude (GameplayEffects|MakeOutgoingSpec _returnvalue "/Game/AbilitySystem/Effects/GE_DamageInstant.GE_DamageInstant_C" 1.0 (GameplayEffects|MakeEffectContext _returnvalue)) "(TagName=\"SetByCaller.Damage.Additive\")" (Variables|Default|GetDamageAdditive)))
      (bind _returnvalue_3 (Ability|GameplayEffect|AssignTagSetbyCallerMagnitude _returnvalue_2 "(TagName=\"SetByCaller.Damage.Multiplier\")" (Variables|Default|GetDamageMultiplier)))
      (GameplayEffects|ApplyGameplayEffectSpecToTarget _returnvalue_3 (.TargetData (Utilities|Struct|BreakGameplayEventData _payload))))))