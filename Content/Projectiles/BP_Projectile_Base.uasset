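; Base projectile Blueprint that applies balance damage with knockback and plays hit cues when it strikes a target with an Ability System Component.
; On pre-hit it applies GE_RangedDamageBalance, passing balance damage and its forward vector as knockback direction via SetByCaller tags.
; It then prints the impact point and fires a GameplayCue chosen by target class: tower, enemy, player or core.
; Regular damage comes from separately prepared GameplayEffects.
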(event EventBeginPlay)

(event Collision|EventActorBeginOverlap
  (params (OtherActor :type Actor%20Object%20Reference)))

(event EventTick
  (params (DeltaSeconds :type Float%20%28single-precision%29)))

(event EventOnProjectilePreHit
  (params (EventData :type Gameplay%20Event%20Data%20Structure%20%28by%20ref%29))
  (bind _target (Utilities|Struct|BreakGameplayEventData EventData))
  (bind (_eventtag _instigator _target_2 _optionalobject _optionalobject2 _contexthandle _instigatortags _targettags _eventmagnitude _targetdata) (Utilities|Struct|BreakGameplayEventData EventData))
  (bind _returnvalue (Transformation|GetActorForwardVector))
  (bind _returnvalue_2 (Ability|GetAbilitySystemComponent _target))
  (bind _returnvalue_3 (Utilities|GetClass _target_2))
  (bind (_x _y _z) (Math|Vector|BreakVector _returnvalue))
  (bind _returnvalue_4 (Ability|TargetData|GetHitResultfromTargetData _targetdata))
  (bind (_bblockinghit _binitialoverlap _time _distance _location _impactpoint _normal _impactnormal) (Collision|BreakHitResult _returnvalue_4))
  (bind _returnvalue_5 (Ability|GameplayCue|MakeGameplayCueParameters :Location _impactpoint :Normal _impactnormal :Instigator _instigator))
  (Utilities|IsValid _returnvalue_2
    (:Is%20Valid
      (Utilities|FlowControl|Sequence
        (:then_0
          ;[1 1 1] Knockback. Note: Damage is dealt by prepared GEs.
          (bind _returnvalue_6 (Ability|GameplayEffect|AssignTagSetbyCallerMagnitude (GameplayEffects|MakeOutgoingSpec _returnvalue_2 "/Game/GameplayEffects/GE_RangedDamageBalance.GE_RangedDamageBalance_C" 1.0 (GameplayEffects|MakeEffectContext _returnvalue_2)) "(TagName=\"SetByCaller.KnockbackDirectionX\")" _x))
          (bind _returnvalue_7 (Ability|GameplayEffect|AssignTagSetbyCallerMagnitude _returnvalue_6 "(TagName=\"SetByCaller.KnockbackDirectionY\")" _y))
          (bind _returnvalue_8 (Ability|GameplayEffect|AssignTagSetbyCallerMagnitude _returnvalue_7 "(TagName=\"SetByCaller.KnockbackDirectionZ\")" _z))
          (bind _returnvalue_9 (Ability|GameplayEffect|AssignTagSetbyCallerMagnitude _returnvalue_8 "(TagName=\"SetByCaller.Balance.Damage\")" (Variables|Default|GetBalanceDamage)))
          (GameplayEffects|ApplyGameplayEffectSpecToTarget (Variables|Default|GetAbilitySystemComponent) _returnvalue_9 _returnvalue_2))
        (:then_1
          ;[1 1 1] Play gameplay cue.
          (Development|PrintString (Utilities|String|ToString(Vector) _impactpoint))
          (if (Utilities|ClassIsChildOf _returnvalue_3 "/Script/mtd.MTD_TowerAsd")
            (GameplayCue|ExecuteGameplayCueOnActor(Burst) _target_2 "(TagName=\"GameplayCue.TowerHit\")" _returnvalue_5)
            (elif (Utilities|ClassIsChildOf _returnvalue_3 "/Game/Characters/Enemies/BP_BaseEnemy.BP_BaseEnemy_C")
              (GameplayCue|ExecuteGameplayCueOnActor(Burst) _target_2 "(TagName=\"GameplayCue.EnemyHit\")" _returnvalue_5)
              (elif (Utilities|ClassIsChildOf _returnvalue_3 "/Game/Characters/Heroes/BP_BasePlayerCharacter.BP_BasePlayerCharacter_C")
                (GameplayCue|ExecuteGameplayCueOnActor(Burst) _target_2 "(TagName=\"GameplayCue.PlayerHit\")" _returnvalue_5)
                (elif (Utilities|ClassIsChildOf _returnvalue_3 "/Game/GameModes/Core/BP_Core.BP_Core_C")
                  (GameplayCue|ExecuteGameplayCueOnActor(Burst) _target_2 "(TagName=\"GameplayCue.CoreHit\")" _returnvalue_5))))))))))

(fn ConstructionScript)