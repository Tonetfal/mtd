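; BP_ManaChest is an interactable chest that bursts into mana tokens in the tower defense mode.
; On interact, it spawns tokens at its transform using the chest token setting from the game mode's selected level definition.
; The tokens are flung in random directions within a speed range.
; Interaction is always allowed, and the chest destroys itself in PostInteract.
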(event EventPostInteract
  (params (Character :type MTD%20Base%20Character%20Object%20Reference) (InteractionID :type Name :default "None"))
  (Actor|DestroyActor))

(fn ConstructionScript)

(fn CanInteract
  (params (Character :type MTD%20Base%20Character%20Object%20Reference) (InteractionID :type Name :default "None"))
  (return true))

(fn Interact
  (params (Character :type MTD%20Base%20Character%20Object%20Reference) (InteractionID :type Name :default "None"))
  (bind _asmtd_tower_defense_mode (Utilities|Casting|CastToMTD_TowerDefenseMode (Game|GetGameMode)))
  (Utilities|IsValid (Variables|/Script/mtd.MTD_TowerDefenseMode|GetSelectedLevelDefinition _asmtd_tower_defense_mode)
    (:Is%20Valid
      (bind _returnvalue (Class|MTDManaToken|SpawnMana self (Transformation|GetActorTransform) (Variables|/Script/mtd.MTD_LevelDefinition|GetChestManaTokens (Variables|/Script/mtd.MTD_TowerDefenseMode|GetSelectedLevelDefinition _asmtd_tower_defense_mode)) (Variables|Default|GetTriggersIgnoreTime)))
      (Class|MTDManaToken|AddRandomDirectionForcetoTokens _returnvalue 7.5e+03 3.25e+04)
      (return true))))