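; Base game mode that ends the match when a core is destroyed.
; On BeginPlay it finds every BP_Core actor and binds to its core-destroyed delegate.
; The first destruction sets a GameOver flag so termination runs only once, then broadcasts OnGameTerminated with an enum result and prints a "Game Over" message.
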(event EventBeginPlay
  (bind _outactors (Actor|GetAllActorsOfClass "/Game/System/BP_Core.BP_Core_C"))
  (for _array_element _outactors
    (EventDispatchers|AssignOnCoreDestroyedDelegate _array_element (EventDispatchers|CreateEvent :!event OnCoreDestroyed))))

(fn ConstructionScript)

(fn OnCoreDestroyed
  (if (not (Variables|Default|GetbGameOver))
    (Variables|Default|SetbGameOver true)
    (Default|CallOnGameTerminated "NewEnumerator0")
    (Development|PrintString "Game Over")))