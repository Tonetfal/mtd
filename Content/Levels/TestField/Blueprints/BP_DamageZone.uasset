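; BP_DamageZone is a test-field volume that damages actors with an Ability System Component while they are inside its box.
; Box overlap events maintain the list of affected actors.
; Every Tick, each target applies an instant damage Gameplay Effect to itself, using SetByCaller magnitudes and a synthesized hit result at its location.
; Damage is not scaled by delta time, so its rate depends on tick frequency.
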(event OnComponentBeginOverlap(Box)
  (params (OverlappedComponent :type Primitive%20Component%20Object%20Reference) (OtherActor :type Actor%20Object%20Reference) (OtherComp :type Primitive%20Component%20Object%20Reference) (OtherBodyIndex :type Integer) (bFromSweep :type Boolean) (SweepResult :type Hit%20Result%20Structure%20%28by%20ref%29))
  (Utilities|IsValid (Ability|GetAbilitySystemComponent OtherActor)
    (:Is%20Valid
      (Utilities|Array|Add (Variables|Default|GetActors) OtherActor))))

(event OnComponentEndOverlap(Box)
  (params (OverlappedComponent :type Primitive%20Component%20Object%20Reference) (OtherActor :type Actor%20Object%20Reference) (OtherComp :type Primitive%20Component%20Object%20Reference) (OtherBodyIndex :type Integer))
  (Utilities|Array|RemoveItem (Variables|Default|GetActors) OtherActor))

(event EventBeginPlay)

(event Collision|EventActorBeginOverlap
  (params (OtherActor :type Actor%20Object%20Reference)))

(event EventTick
  (params (DeltaSeconds :type Float%20%28single-precision%29))
  (for _array_element (Variables|Default|GetActors)
    (Utilities|IsValid (Ability|GetAbilitySystemComponent _array_element)
      (:Is%20Valid
        (bind _output_get (Variables|Default|SetEffectContext (GameplayEffects|MakeEffectContext (Ability|GetAbilitySystemComponent _array_element))))
        (Class|AbilitySystemBlueprintLibrary|EffectContextAddHitResult _output_get (Collision|MakeHitResult true false 0.0 0.0 (Transformation|GetActorLocation _array_element) "0, 0, 0" "0,0,1" "0,0,1" 0 _array_element) false)
        (bind _returnvalue (Ability|GameplayEffect|AssignTagSetbyCallerMagnitude (GameplayEffects|MakeOutgoingSpec (Ability|GetAbilitySystemComponent _array_element) "/Game/GameplayEffects/GE_DamageInstant_Regular.GE_DamageInstant_Regular_C" 1.0 (Variables|Default|GetEffectContext)) "(TagName=\"SetByCaller.Damage.Base\")" (Variables|Default|GetDamage)))
        (bind _returnvalue_2 (Ability|GameplayEffect|AssignTagSetbyCallerMagnitude _returnvalue "(TagName=\"SetByCaller.Damage.Additive\")" 0.0))
        (bind _returnvalue_3 (Ability|GameplayEffect|AssignTagSetbyCallerMagnitude _returnvalue_2 "(TagName=\"SetByCaller.Damage.Multiplier\")" 1.0))
        (GameplayEffects|ApplyGameplayEffectSpecToSelf (Ability|GetAbilitySystemComponent _array_element) _returnvalue_3)))))

(fn ConstructionScript)