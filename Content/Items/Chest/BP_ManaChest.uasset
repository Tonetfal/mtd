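; Mana chest item that any character can interact with to burst it into mana tokens.
; On interaction it synchronously loads the default mana token data asset and spawns tokens for its Mana amount at its transform.
; The tokens get a launch velocity and briefly ignore triggers.
; The chest then destroys itself, even if the data cast fails.
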(event EventBeginPlay)

(event Collision|EventActorBeginOverlap
  (params (OtherActor :type Actor%20Object%20Reference)))

(event EventTick
  (params (DeltaSeconds :type Float%20%28single-precision%29)))

(event EventInteract
  (params (Character :type MTD%20Base%20Character%20Object%20Reference))
  (Utilities|FlowControl|Sequence
    (:then_0
      (bind _returnvalue (Utilities|LoadAssetBlocking "/Game/Items/Mana/MTD_Default.MTD_Default"))
      (bind _asmtd_mana_tokens_data (Utilities|Casting|CastToMTD_ManaTokensData _returnvalue))
      (bind _returnvalue_2 (Class|MTDManaToken|SpawnMana self (Transformation|GetActorTransform) (Variables|Default|GetMana) (Variables|/Script/mtd.MTD_ManaTokensData|GetData _asmtd_mana_tokens_data)))
      (Class|MTDManaToken|GiveStartVelocitytoTokens _returnvalue_2 2.5e+03 5e+03)
      (for _array_element _returnvalue_2
        (Class|MTDFloatingToken|IgnoreTriggersfor _array_element (Variables|Default|GetSecondsToIgnoreTriggersAfterSpawnFor))))
    (:then_1
      (Actor|DestroyActor))))

(event EventTryInteract
  (params (Character :type MTD%20Base%20Character%20Object%20Reference))
  (bind _bresult (CallFunction|CanInteract Character))
  (if _bresult
    (CallFunction|Interact Character)))

(fn ConstructionScript)

(fn CanInteract
  (params (Character :type MTD%20Base%20Character%20Object%20Reference))
  (return true))