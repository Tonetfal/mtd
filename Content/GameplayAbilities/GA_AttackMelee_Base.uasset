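; Base melee attack gameplay ability that turns MeleeHit gameplay events into knockback, damage and impact feedback.
; On each hit, it applies GE_DamageBalance with the avatar-to-target vector as SetByCaller knockback direction, then GE_DamageInstant with additive and multiplier damage.
; Knockback goes first so a death animation can cancel the hit animation.
; It then executes a gameplay cue at the impact point, chosen by target class: tower, enemy, player or core.
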(event Ability|EventActivateAbility
  (bind _returnvalue (Ability|GetAbilitySystemComponentfromActorInfo))
  (bind _returnvalue_2 (GameplayEffects|MakeEffectContext _returnvalue))
  (|CallParentFunction)
  (bind _payload (Ability|Tasks|WaitGameplayEvent "(TagName=\"Gameplay.Event.MeleeHit\")" 0)
    (:EventReceived
      (Variables|Private|SetPayload _payload)
      (Utilities|FlowControl|Sequence
        (:then_0
          ;[1 1 1] Damage and knockback hit actor. Knockback first because it causes the actor to play its hit animation, while damage may trigger the death animation that should cancel the hit one.
          (bind _returnvalue_3 (Ability|GameplayEffect|AssignTagSetbyCallerMagnitude (GameplayEffects|MakeOutgoingSpec _returnvalue "/Game/GameplayEffects/GE_DamageBalance.GE_DamageBalance_C" 1.0 _returnvalue_2) "(TagName=\"SetByCaller.KnockbackDirectionX\")" (.x (- (Transformation|GetActorLocation (.Target (Utilities|Struct|BreakGameplayEventData (Variables|Private|GetPayload)))) (Transformation|GetActorLocation (Ability|GetAvatarActorfromActorInfo))))))
          (bind _returnvalue_4 (Ability|GameplayEffect|AssignTagSetbyCallerMagnitude _returnvalue_3 "(TagName=\"SetByCaller.KnockbackDirectionY\")" (.y (- (Transformation|GetActorLocation (.Target (Utilities|Struct|BreakGameplayEventData (Variables|Private|GetPayload)))) (Transformation|GetActorLocation (Ability|GetAvatarActorfromActorInfo))))))
          (bind _returnvalue_5 (Ability|GameplayEffect|AssignTagSetbyCallerMagnitude _returnvalue_4 "(TagName=\"SetByCaller.KnockbackDirectionZ\")" (.z (- (Transformation|GetActorLocation (.Target (Utilities|Struct|BreakGameplayEventData (Variables|Private|GetPayload)))) (Transformation|GetActorLocation (Ability|GetAvatarActorfromActorInfo))))))
          (bind _returnvalue_6 (Ability|GameplayEffect|AssignTagSetbyCallerMagnitude (GameplayEffects|MakeOutgoingSpec _returnvalue "/Game/GameplayEffects/GE_DamageInstant.GE_DamageInstant_C" 1.0 _returnvalue_2) "(TagName=\"SetByCaller.Damage.Additive\")" (Variables|Default|GetDamageAdditive)))
          (bind _returnvalue_7 (Ability|GameplayEffect|AssignTagSetbyCallerMagnitude _returnvalue_6 "(TagName=\"SetByCaller.Damage.Multiplier\")" (Variables|Default|GetDamageMultiplier)))
          (GameplayEffects|ApplyGameplayEffectSpecToTarget _returnvalue_5 (.TargetData (Utilities|Struct|BreakGameplayEventData (Variables|Private|GetPayload))))
          (GameplayEffects|ApplyGameplayEffectSpecToTarget _returnvalue_7 (.TargetData (Utilities|Struct|BreakGameplayEventData (Variables|Private|GetPayload)))))
        (:then_1
          ;[1 1 1] Play gameplay cue.
          (if (Utilities|ClassIsChildOf (Utilities|GetClass (.Target (Utilities|Struct|BreakGameplayEventData (Variables|Private|GetPayload)))) "/Script/mtd.MTD_TowerAsd")
            (Class|GameplayAbility|ExecuteGameplayCuewithParams "(TagName=\"GameplayCue.TowerHit\")" (Ability|GameplayCue|MakeGameplayCueParameters :EffectContext _returnvalue_2 :Location (.ImpactPoint (Collision|BreakHitResult (Ability|TargetData|GetHitResultfromTargetData (.TargetData (Utilities|Struct|BreakGameplayEventData (Variables|Private|GetPayload)))))) :Normal (.ImpactNormal (Collision|BreakHitResult (Ability|TargetData|GetHitResultfromTargetData (.TargetData (Utilities|Struct|BreakGameplayEventData (Variables|Private|GetPayload)))))) :Instigator (.Instigator (Utilities|Struct|BreakGameplayEventData (Variables|Private|GetPayload)))))
            (elif (Utilities|ClassIsChildOf (Utilities|GetClass (.Target (Utilities|Struct|BreakGameplayEventData (Variables|Private|GetPayload)))) "/Game/Characters/Enemies/BP_BaseEnemy.BP_BaseEnemy_C")
              (Class|GameplayAbility|ExecuteGameplayCuewithParams "(TagName=\"GameplayCue.PlayerHit\")" (Ability|GameplayCue|MakeGameplayCueParameters :EffectContext _returnvalue_2 :Location (.ImpactPoint (Collision|BreakHitResult (Ability|TargetData|GetHitResultfromTargetData (.TargetData (Utilities|Struct|BreakGameplayEventData (Variables|Private|GetPayload)))))) :Normal (.ImpactNormal (Collision|BreakHitResult (Ability|TargetData|GetHitResultfromTargetData (.TargetData (Utilities|Struct|BreakGameplayEventData (Variables|Private|GetPayload)))))) :Instigator (.Instigator (Utilities|Struct|BreakGameplayEventData (Variables|Private|GetPayload)))))
              (elif (Utilities|ClassIsChildOf (Utilities|GetClass (.Target (Utilities|Struct|BreakGameplayEventData (Variables|Private|GetPayload)))) "/Game/Characters/Heroes/BP_BasePlayerCharacter.BP_BasePlayerCharacter_C")
                (Class|GameplayAbility|ExecuteGameplayCuewithParams "(TagName=\"GameplayCue.EnemyHit\")" (Ability|GameplayCue|MakeGameplayCueParameters :EffectContext _returnvalue_2 :Location (.ImpactPoint (Collision|BreakHitResult (Ability|TargetData|GetHitResultfromTargetData (.TargetData (Utilities|Struct|BreakGameplayEventData (Variables|Private|GetPayload)))))) :Normal (.ImpactNormal (Collision|BreakHitResult (Ability|TargetData|GetHitResultfromTargetData (.TargetData (Utilities|Struct|BreakGameplayEventData (Variables|Private|GetPayload)))))) :Instigator (.Instigator (Utilities|Struct|BreakGameplayEventData (Variables|Private|GetPayload)))))
                (elif (Utilities|ClassIsChildOf (Utilities|GetClass (.Target (Utilities|Struct|BreakGameplayEventData (Variables|Private|GetPayload)))) "/Game/GameModes/Core/BP_Core.BP_Core_C")
                  (Class|GameplayAbility|ExecuteGameplayCuewithParams "(TagName=\"GameplayCue.CoreHit\")" (Ability|GameplayCue|MakeGameplayCueParameters :EffectContext _returnvalue_2 :Location (.ImpactPoint (Collision|BreakHitResult (Ability|TargetData|GetHitResultfromTargetData (.TargetData (Utilities|Struct|BreakGameplayEventData (Variables|Private|GetPayload)))))) :Normal (.ImpactNormal (Collision|BreakHitResult (Ability|TargetData|GetHitResultfromTargetData (.TargetData (Utilities|Struct|BreakGameplayEventData (Variables|Private|GetPayload)))))) :Instigator (.Instigator (Utilities|Struct|BreakGameplayEventData (Variables|Private|GetPayload))))))))))))))