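; Target dummy actor that registers as a sight stimulus so towers see it and displays damage taken per second as floating text.
; BeginPlay also registers it as a GameFrameworkComponentManager receiver for plugin-added components.
; OnHealthDecrease accumulates lost health and starts a one-second timer if none is pending.
; DisplayDPS then spawns colored, offset text through any SFT_FloatingTextComponent found on the actor and resets the total and timer.
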(event EventBeginPlay
  (Utilities|FlowControl|Sequence
    (:then_0
      ;[1 1 1] Add plugins.
      (Class|GameFrameworkComponentManager|AddReceiver (Subsystems|GetGameFrameworkComponentManager)))
    (:then_1
      ;[1 1 1] Make towers see it.
      (Class|AIPerceptionStimuliSourceComponent|RegisterforSense (Variables|Default|GetAIPerceptionStimuliSource) "/Script/AIModule.AISense_Sight"))))

(event Collision|EventActorBeginOverlap
  (params (OtherActor :type Actor%20Object%20Reference)))

(event EventTick
  (params (DeltaSeconds :type Float%20%28single-precision%29)))

(event EventOnHealthDecrease
  (params (LostHealth :type Float%20%28single-precision%29))
  (Utilities|FlowControl|Sequence
    (:then_0
      ;[1 1 1] Setup DisplayDPS timer handle to play after a second.
      (if (not (Utilities|Time|IsValidTimerHandle (Variables|Default|GetDpsTimerHandle)))
        (bind _returnvalue (Utilities|Time|SetTimerbyFunctionName 0 "DisplayDPS" 1.0))
        (Variables|Default|SetDpsTimerHandle _returnvalue)))
    (:then_1
      ;[1 1 1] Accumulate damage.
      (Variables|Default|SetDamageSinceLastDisplay (+ (Variables|Default|GetDamageSinceLastDisplay) LostHealth)))))

(fn ConstructionScript)

(fn GetFloatingTextPosition
  (return (+ (Transformation|GetActorLocation) (Variables|Default|GetDpsTextOffset))))

(fn DisplayDPS
  (bind _returnvalue (Actor|GetComponentbyClass "/Script/ScreenFloatingTextRuntime.SFT_FloatingTextComponent"))
  (Utilities|FlowControl|Sequence
    (:then_0
      ;[1 1 1] Display the DPS.
      (Utilities|IsValid _returnvalue
        (:Is%20Valid
          (bind (_outfloatingtextactor _outtextblock) (Class|SFTFloatingTextComponent|SpawnFloatingText _returnvalue (CallFunction|GetFloatingTextPosition)))
          (Utilities|FlowControl|Sequence
            (:then_0
              (Utilities|IsValid _outfloatingtextactor
                (:Is%20Valid
                  (Class|SFTFloatingTextActor|PostInitialize _outfloatingtextactor))))
            (:then_1
              (Utilities|IsValid _outtextblock
                (:Is%20Valid
                  (Variables|/Script/UMG.TextBlock|SetText _outtextblock (Utilities|Text|FormatText "{DPS}" (Variables|Default|GetDamageSinceLastDisplay)))
                  (Appearance|SetColorandOpacity _outtextblock (Utilities|Struct|MakeSlateColor (Variables|Default|GetDpsTextColor)) :!class /Script/UMG.TextBlock))))))))
    (:then_1
      ;[1 1 1] Reset DPS state.
      (Utilities|Time|InvalidateTimerHandle (Variables|Default|GetDpsTimerHandle))
      (Variables|Default|SetDamageSinceLastDisplay 0.0))))