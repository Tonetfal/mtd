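; BP_Core is the tower defense core, an actor with health that is destroyed when that health runs out.
; On BeginPlay it grants GA_Death_Core, tries to activate all its abilities with a debug print, and applies GE_CoreStats with SetByCaller health from the selected level definition.
; It then binds its HealthComponent to the ability system.
; Health drops are broadcast through a delegate, and zero health broadcasts destruction and destroys the actor.
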(event EventBeginPlay
  (bind _returnvalue (Game|GetGameMode))
  (bind _returnvalue_2 (Class|MTDCore|GetMtdAbilitySystemComponent))
  ;[1 1 1] Cache and check validness.
  (Utilities|IsValid _returnvalue_2
    (:Is%20Valid
      (Variables|Default|SetAbilitySystemComponent _returnvalue_2)
      (Utilities|IsValid _returnvalue
        (:Is%20Valid
          (bind _asbp_tower_defense_mode (Utilities|Casting|CastToBP_TowerDefenseMode _returnvalue))
          (Utilities|IsValid (Variables|/Script/mtd.MTD_TowerDefenseMode|GetSelectedLevelDefinition _asbp_tower_defense_mode)
            (:Is%20Valid
              (Variables|Default|SetLevelDefinition (Variables|/Script/mtd.MTD_TowerDefenseMode|GetSelectedLevelDefinition _asbp_tower_defense_mode))
              ;[1 1 1] Give the ability to die.
              (GameplayAbilities|GiveAbility (Variables|Default|GetAbilitySystemComponent) "/Game/Gameplay/Core/GA_Death_Core.GA_Death_Core_C" 0 -1)
              (bind _outabilityhandles (Class|AbilitySystemComponent|GetAllAbilities (Variables|Default|GetAbilitySystemComponent)))
              (for _array_element _outabilityhandles
                (bind _returnvalue_3 (Class|AbilitySystemComponent|TryActivateAbility (Variables|Default|GetAbilitySystemComponent) _array_element true))
                (Development|PrintString (Utilities|String|Append "Try activate Death on Core: " (Utilities|String|ToString(Boolean) _returnvalue_3)) true true "(R=1.000000,G=0.000000,B=0.160469,A=1.000000)" 1e+01))
              ;[1 1 1] Modify default attributes.
              (bind _returnvalue_4 (Ability|GameplayEffect|AssignTagSetbyCallerMagnitude (GameplayEffects|MakeOutgoingSpec (Variables|Default|GetAbilitySystemComponent) "/Game/GameplayEffects/GE_CoreStats.GE_CoreStats_C" 1.0 (GameplayEffects|MakeEffectContext (Variables|Default|GetAbilitySystemComponent))) "(TagName=\"SetByCaller.MaxHealth\")" (Math|Conversions|ToFloat(Integer) (Variables|/Script/mtd.MTD_LevelDefinition|GetCoreHealth (Variables|Default|GetLevelDefinition)))))
              (bind _returnvalue_5 (Ability|GameplayEffect|AssignTagSetbyCallerMagnitude _returnvalue_4 "(TagName=\"SetByCaller.Health\")" (Math|Conversions|ToFloat(Integer) (Variables|/Script/mtd.MTD_LevelDefinition|GetCoreHealth (Variables|Default|GetLevelDefinition)))))
              (GameplayEffects|ApplyGameplayEffectSpecToSelf (Variables|Default|GetAbilitySystemComponent) _returnvalue_5)
              ;[1 1 1] Initialize health component.
              (Class|MTDHealthComponent|InitializewithAbilitySystem (Variables|Default|GetHealthComponent) (Variables|Default|GetAbilitySystemComponent)))))))))

(event EventOnCoreDestroyed
  (params (OwningActor :type Actor%20Object%20Reference))
  (Default|CallOnCoreDestroyedDelegate)
  (Actor|DestroyActor))

(event EventOnCoreHealthChanged
  (params (InHealthComponent :type MTD%20Health%20Component%20Object%20Reference) (OldValue :type Float%20%28single-precision%29) (NewValue :type Float%20%28single-precision%29) (InInstigator :type Actor%20Object%20Reference))
  (if (< NewValue OldValue)
    (Default|CallOnCoreHealthChangedDelegate OldValue NewValue)
    (if (== NewValue 0.0)
      (Default|CallOnCoreDestroyedDelegate)
      (Actor|DestroyActor))))

(event EventEndPlay
  (params (EndPlayReason :type EEndPlayReason%20Enum :default "Destroyed"))
  (Class|MTDHealthComponent|UninitializefromAbilitySystem (Variables|Default|GetHealthComponent)))

(fn ConstructionScript)