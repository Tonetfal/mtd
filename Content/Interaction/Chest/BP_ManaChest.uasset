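; BP_ManaChest is an interactable chest that bursts into mana tokens when used and then removes itself.
; It always allows interaction, then synchronously loads the default mana tokens data asset and spawns tokens from its table for its Mana amount.
; The tokens spawn at the chest's transform with a trigger ignore time and receive a starting velocity.
; PostInteract destroys the actor.
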(event EventPostInteract
  (params (Character :type MTD%20Base%20Character%20Object%20Reference) (InteractionID :type Name :default "None"))
  (Actor|DestroyActor))

(fn ConstructionScript)

(fn CanInteract
  (params (Character :type MTD%20Base%20Character%20Object%20Reference) (InteractionID :type Name :default "None"))
  (return true))

(fn Interact
  (params (Character :type MTD%20Base%20Character%20Object%20Reference) (InteractionID :type Name :default "None"))
  (bind _returnvalue (Utilities|LoadAssetBlocking "/Game/Interaction/Mana/ManaTokensData_Default.ManaTokensData_Default"))
  (bind _asmtd_mana_tokens_data (Utilities|Casting|CastToMTD_ManaTokensData _returnvalue))
  (bind _returnvalue_2 (Class|MTDManaToken|SpawnMana self (Transformation|GetActorTransform) (Variables|Default|GetMana) (Variables|/Script/mtd.MTD_ManaTokensData|GetData _asmtd_mana_tokens_data) (Variables|Default|GetTriggersIgnoreTime)))
  (Class|MTDManaToken|GiveStartVelocitytoTokens _returnvalue_2 7.5e+03 2.5e+04)
  (return true))