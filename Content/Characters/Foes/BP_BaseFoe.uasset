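; Base Blueprint for foe characters, extending its parent's health, death and loot behavior.
; Registers as a GameFrameworkComponentManager receiver and starts with a hidden status bar, whose visibility changes gate health bar progress and text updates.
; Goods drops also spawn mana tokens from FoeData, flung in random directions.
; Death finishes with a timeline that rescales the mesh before destroying the controller and actor.
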(event EventOnDeathFinished
  (params (OwningActor :type Actor%20Object%20Reference))
  (bind _returnvalue (Pawn|GetController))
  ;[1 1 1] Override death event. Scale down before destroying the actor.
  (|CallParentFunction OwningActor)
  (bind _scaling (Timeline|Timeline PlayFromStart)
    (:Update
      (Transformation|SetRelativeScale3D (Variables|Character|GetMesh) (Math|Conversions|ToVector(Float) _scaling)))
    (:Finished
      (Utilities|IsValid _returnvalue
        (:Is%20Valid
          (Actor|DestroyActor _returnvalue))
        (:Is%20Not%20Valid
          _))
      (Actor|DestroyActor))))

(event EventOnHealthChanged
  (params (InHealthComponent :type MTD%20Health%20Component%20Object%20Reference) (OldValue :type Float%20%28single-precision%29) (NewValue :type Float%20%28single-precision%29) (InInstigator :type Actor%20Object%20Reference))
  (|CallParentFunction InHealthComponent OldValue NewValue InInstigator)
  (CallFunction|UpdateHealthWidgetProgress))

(event EventBeginPlay
  (bind _statusbar (Variables|Default|GetStatusBar))
  (bind _returnvalue (UserInterface|GetWidget _statusbar))
  (Utilities|FlowControl|Sequence
    (:then_0
      (Utilities|FlowControl|Sequence
        (:then_0
          ;[1 1 1] Add plugins.
          (Class|GameFrameworkComponentManager|AddReceiver (Subsystems|GetGameFrameworkComponentManager)))
        (:then_1
          ;[1 1 1] Setup status bar.
          (Utilities|IsValid _returnvalue
            (:Is%20Valid
              (EventDispatchers|AssignOnVisibilityChanged _returnvalue (EventDispatchers|CreateEvent :!event OnHealthWidgetVisibilityChanged))
              (Widget|SetRenderOpacity _returnvalue 0.0)
              (Widget|SetVisibility _returnvalue "Hidden"))))))
    (:then_1
      (|CallParentFunction))))

(event EventDropGoods
  (|CallParentFunction)
  (CallFunction|DropMana))

(fn ConstructionScript
  (|CallParentFunction))

(fn DropMana
  (bind _foedata (Variables|Default|GetFoeData))
  (Utilities|IsValid _foedata
    (:Is%20Valid
      (bind _returnvalue (Class|MTDManaToken|SpawnMana self (Transformation|GetActorTransform) (Variables|/Script/mtd.MTD_FoeData|GetManaTokens _foedata) (Variables|MTD|Mana|GetTriggersIgnoreTime)))
      (Class|MTDManaToken|AddRandomDirectionForcetoTokens _returnvalue 7.5e+03 1.25e+04))))

(fn OnHealthWidgetVisibilityChanged
  (params (InVisibility :type ESlateVisibility%20Enum :default "Visible"))
  (switch Utilities|FlowControl|Switch|SwitchonESlateVisibility InVisibility
    (:Visible
      (Variables|MTD|FrontEnd|SetbShouldHealthWidgetUpdate true)
      (CallFunction|UpdateHealthWidgetProgress))
    (:Collapsed
      (Variables|MTD|FrontEnd|SetbShouldHealthWidgetUpdate false :!label _label))
    (:Hidden
      (goto _label))
    (:HitTestInvisible
      (goto _label))
    (:SelfHitTestInvisible
      (goto _label))))

(fn UpdateHealthWidgetProgress
  (bind _healthcomponent (Variables|Default|GetHealthComponent))
  (bind _statusbar (Variables|Default|GetStatusBar))
  (bind _returnvalue (UserInterface|GetWidget _statusbar))
  (if (Variables|MTD|FrontEnd|GetbShouldHealthWidgetUpdate)
    (Utilities|IsValid _returnvalue
      (:Is%20Valid
        (bind _aswbp_foe_status_bar (Utilities|Casting|CastToWBP_FoeStatusBar _returnvalue))
        (Default|SetProgress (Variables|/Game/UI/Widgets/WBP_FoeStatusBar.WBP_FoeStatusBar_C|GetHealthBar _aswbp_foe_status_bar) (Class|MTDHealthComponent|GetHealthNormilized _healthcomponent))
        (Default|SetText (Variables|/Game/UI/Widgets/WBP_FoeStatusBar.WBP_FoeStatusBar_C|GetHealthBar _aswbp_foe_status_bar) (Class|MTDHealthComponent|GetHealth _healthcomponent) (Class|MTDHealthComponent|GetMaxHealth _healthcomponent))))))