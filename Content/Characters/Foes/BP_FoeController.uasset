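; BP_FoeController is a controller for foe pawns that manages its AI perception stimuli source as it possesses and releases them.
; On possess, it runs the parent logic, then registers the stimuli source for sight if the pawn derives from BP_BaseFoe.
; An invalid pawn prints a wrong-type message, while a valid pawn of another class is silently skipped.
; On unpossess, it unregisters the source from the perception system.
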(event EventUnPossess
  (params (UnpossessedPawn :type Pawn%20Object%20Reference))
  (Class|AIPerceptionStimuliSourceComponent|UnregisterfromPerceptionSystem (Variables|Default|GetAI%20Perception%20Stimuli%20Source)))

(event EventPossess
  (params (PossessedPawn :type Pawn%20Object%20Reference))
  (|CallParentFunction PossessedPawn)
  (Utilities|IsValid PossessedPawn
    (:Is%20Valid
      (if (Utilities|ClassIsChildOf (Utilities|GetClass PossessedPawn) "/Game/Characters/Foes/BP_BaseFoe.BP_BaseFoe_C")
        ;[1 1 1] Register for sight sense.
        (Class|AIPerceptionStimuliSourceComponent|RegisterforSense (Variables|Default|GetAI%20Perception%20Stimuli%20Source) "/Script/AIModule.AISense_Sight")))
    (:Is%20Not%20Valid
      (Development|PrintString (Utilities|String|Append "[" (Utilities|GetDisplayName PossessedPawn) "] is not of type BP_BaseEnemy")))))

(fn ConstructionScript)