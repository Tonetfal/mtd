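; Base melee attack gameplay ability that turns strike events into damage and hit feedback.
; On activation it waits for Action.MeleeStrike gameplay events, whose payload carries the target data.
; Each event applies an instant damage effect to those targets, with additive and multiplier values set by caller.
; It then fires the sword-hit gameplay cue, placed using the first hit result's location plus impact point.
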(event Ability|EventActivateAbility
  (bind _returnvalue (Ability|GetAbilitySystemComponentfromActorInfo))
  (bind _returnvalue_2 (GameplayEffects|MakeEffectContext _returnvalue))
  (bind _payload (Ability|Tasks|WaitGameplayEvent "(TagName=\"Action.MeleeStrike\")" 0)
    (:EventReceived
      (Variables|Private|SetPayload _payload)
      (Utilities|FlowControl|Sequence
        (:then_0
          ;[1 1 1] Damage.
          (bind _returnvalue_3 (Ability|GameplayEffect|AssignTagSetbyCallerMagnitude (GameplayEffects|MakeOutgoingSpec _returnvalue "/Game/GameplayEffects/GE_DamageInstant.GE_DamageInstant_C" 1.0 _returnvalue_2) "(TagName=\"SetByCaller.Damage.Additive\")" (Variables|Default|GetDamageAdditive)))
          (bind _returnvalue_4 (Ability|GameplayEffect|AssignTagSetbyCallerMagnitude _returnvalue_3 "(TagName=\"SetByCaller.Damage.Multiplier\")" (Variables|Default|GetDamageMultiplier)))
          (GameplayEffects|ApplyGameplayEffectSpecToTarget _returnvalue_4 (.TargetData (Utilities|Struct|BreakGameplayEventData (Variables|Private|GetPayload)))))
        (:then_1
          (Class|GameplayAbility|ExecuteGameplayCuewithParams "(TagName=\"GameplayCue.Weapon.Sword.Hit\")" (Ability|GameplayCue|MakeGameplayCueParameters :EffectContext _returnvalue_2 :Location (+ (.Location (Collision|BreakHitResult (Ability|TargetData|GetHitResultfromTargetData (.TargetData (Utilities|Struct|BreakGameplayEventData (Variables|Private|GetPayload)))))) (.ImpactPoint (Collision|BreakHitResult (Ability|TargetData|GetHitResultfromTargetData (.TargetData (Utilities|Struct|BreakGameplayEventData (Variables|Private|GetPayload))))))) :Normal (.ImpactNormal (Collision|BreakHitResult (Ability|TargetData|GetHitResultfromTargetData (.TargetData (Utilities|Struct|BreakGameplayEventData (Variables|Private|GetPayload)))))) :Instigator (.Instigator (Utilities|Struct|BreakGameplayEventData (Variables|Private|GetPayload))))))))))