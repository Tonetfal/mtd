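; Gameplay Ability that starts a wave in the tower defense game mode.
; On activation it casts the game mode to BP_TowerDefenseMode, calls StartWave, and ends immediately.
; CanActivateAbility allows activation only when that game mode is active, printing a failure message if a different mode is in use.
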(event Ability|EventActivateAbility
  (|CallParentFunction)
  (bind _asbp_tower_defense_mode (Utilities|Casting|CastToBP_TowerDefenseMode (Game|GetGameMode)))
  (Class|MTDTowerDefenseMode|StartWave _asbp_tower_defense_mode)
  (Ability|EndAbility))

(event Ability|EventOnEndAbility
  (params (bWasCancelled :type Boolean))
  (|CallParentFunction bWasCancelled) ; This node is disabled and will not be called.\nDrag off pins to build functionality.
)

(fn K2CanActivateAbility
  (params (ActorInfo :type Gameplay%20Ability%20Actor%20Info%20Structure) (Handle :type Gameplay%20Ability%20Spec%20Handle%20Structure))
  (bind _returnvalue (Game|GetGameMode))
  (Utilities|IsValid _returnvalue
    (:Is%20Valid
      (Utilities|Casting|CastToBP_TowerDefenseMode _returnvalue
        (:then
          (return "" true))
        (:CastFailed
          (Development|PrintString "Failed to activate GA_StartWave ability has been granted while TD GM is not the case." true true "(R=1.000000,G=0.000000,B=0.000000,A=1.000000)" 1e+01)
          (return "" false))))))