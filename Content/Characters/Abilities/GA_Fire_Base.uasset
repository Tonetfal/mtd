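; Base ranged-fire gameplay ability that plays a random montage and launches the equipped weapon's projectile on the Animation.Fire event, ending when the montage blends out or aborts.
; FireProjectile caches weapon, team and camera data, then spawns the projectile at the fire point.
; Only players compute direction, using a camera trace's first hit or camera forward if it is a player, tower or miss.
; Weapon speed, on-hit effects and a ranged damage spec are passed into the projectile.
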(event Ability|EventActivateAbility
  (bind _returnvalue (Ability|GetAvatarActorfromActorInfo))
  (bind _returnvalue_2 (Class|MTDGameplayAbility|GetRandomAbilityAnimMontage _returnvalue))
  (bind _returnvalue_3 (Ability|CommitAbility))
  (if _returnvalue_3
    (Utilities|IsValid _returnvalue_2
      (:Is%20Valid
        (|PlayMontageandWaitProxy "None" _returnvalue_2 1.0 "None" false 1.0 0.0
          (:then
            (Ability|Tasks|WaitGameplayEvent "(TagName=\"Animation.Fire\")" 0
              (:EventReceived
                (CallFunction|FireProjectile))))
          (:OnBlendOut
            (Ability|EndAbility :!label _label))
          (:OnInterrupted
            (goto _label))
          (:OnCancelled
            (goto _label)))))))

(fn FireProjectile
  (Utilities|FlowControl|Sequence
    (:then_0
      ;[1 1 1] Cache data.
      (bind _output_get (LocalVariables|SetAvatar (Ability|GetAvatarActorfromActorInfo)))
      (bind _asbp_base_character (Utilities|Casting|CastToBP_BaseCharacter _output_get))
      (LocalVariables|SetBaseCharacter _asbp_base_character)
      (bind _asmtd_ranged_weapon_instance (Utilities|Casting|CastToMTD_RangedWeaponInstance (Class|MTDEquipmentManagerComponent|GetEquipmentInstance (Variables|/Game/Characters/BP_BaseCharacter.BP_BaseCharacter_C|GetMTD_EquipmentManager (LocalVariables|GetBaseCharacter)))))
      (LocalVariables|SetRangedWeaponInstance _asmtd_ranged_weapon_instance)
      (Utilities|IsValid (Pawn|GetController (LocalVariables|GetBaseCharacter))
        (:Is%20Valid
          (Utilities|IsValid (Actor|GetComponentbyClass (Pawn|GetController (LocalVariables|GetBaseCharacter)) "/Script/mtd.MTD_TeamComponent")
            (:Is%20Valid
              (LocalVariables|SetTeamComponent (Actor|GetComponentbyClass (Pawn|GetController (LocalVariables|GetBaseCharacter)) "/Script/mtd.MTD_TeamComponent"))
              (Utilities|IsValid (Actor|GetComponentbyClass (LocalVariables|GetBaseCharacter) "/Script/Engine.CameraComponent")
                (:Is%20Valid
                  (bind _output_get_2 (LocalVariables|SetCamera (Actor|GetComponentbyClass (LocalVariables|GetBaseCharacter) "/Script/Engine.CameraComponent")))
                  (LocalVariables|SetCameraWorldLocation (Transformation|GetWorldLocation _output_get_2))
                  (LocalVariables|SetCameraWorldForwardVector (Math|Vector|GetForwardVector _output_get_2))
                  (Utilities|IsValid (Variables|/Script/mtd.MTD_RangedWeaponInstance|GetProjectileData (LocalVariables|GetRangedWeaponInstance))
                    (:Is%20Valid
                      (if (Utilities|IsValidClass (Variables|/Script/mtd.MTD_FireData|GetProjectileClass (Variables|/Script/mtd.MTD_RangedWeaponInstance|GetProjectileData (LocalVariables|GetRangedWeaponInstance))))
                        (LocalVariables|SetProjectileClass (Variables|/Script/mtd.MTD_FireData|GetProjectileClass (Variables|/Script/mtd.MTD_RangedWeaponInstance|GetProjectileData (LocalVariables|GetRangedWeaponInstance))))
                        (LocalVariables|SetProjectileParameters (Variables|/Script/mtd.MTD_FireData|GetProjectileParameters (Variables|/Script/mtd.MTD_RangedWeaponInstance|GetProjectileData (LocalVariables|GetRangedWeaponInstance))))
                        (LocalVariables|SetFirePointWorldPosition (Class|MTDRangedWeaponInstance|GetFirePointWorldPosition (LocalVariables|GetRangedWeaponInstance)))
                        (LocalVariables|SetbCached true)))))))))))
    (:then_1
      ;[1 1 1] Check if cached successfully.
      (if (not (LocalVariables|GetbCached))
        (Development|PrintString "Something couldn't be cached successfully." true true "(R=1.000000,G=0.000000,B=0.016606,A=1.000000)" 1e+01)
        (else
          (Utilities|FlowControl|Sequence
            (:then_0
              ;[1 1 1] Spawn actor.
              (bind _returnvalue (Game|SpawnActorfromClass (LocalVariables|GetProjectileClass) (Math|Transform|MakeTransform (LocalVariables|GetFirePointWorldPosition) (Transformation|GetActorRotation (Ability|GetAvatarActorfromActorInfo)) "1.000000,1.000000,1.000000") "AlwaysSpawn" (LocalVariables|GetBaseCharacter) (LocalVariables|GetBaseCharacter)))
              (LocalVariables|SetProjectile _returnvalue))
            (:then_1
              ;[1 1 1] Compute fire point. (For players only)
              (if (Utilities|ClassIsChildOf (Utilities|GetClass (LocalVariables|GetAvatar)) "/Game/Characters/Heroes/BP_BasePlayerCharacter.BP_BasePlayerCharacter_C")
                (bind (_outhits _returnvalue_2) (Collision|MultiLineTraceByChannel (LocalVariables|GetCameraWorldLocation) (+ (LocalVariables|GetCameraWorldLocation) (* (LocalVariables|GetCameraWorldForwardVector) (Variables|MTD|Fire|GetAimTraceLength))) "TraceTypeQuery1" false 0 (select (Variables|MTD|Fire|GetDebugAimTrace) "ForOneFrame" "None")))
                (if _returnvalue_2
                  (bind _array_element (Utilities|Array|ForEachLoopwithBreak _outhits :!label _label)
                    (:LoopBody
                      (if (not (or (Utilities|ClassIsChildOf (Utilities|GetClass (.HitActor (Collision|BreakHitResult _array_element))) "/Game/Characters/Heroes/BP_BasePlayerCharacter.BP_BasePlayerCharacter_C") (Utilities|ClassIsChildOf (Utilities|GetClass (.HitActor (Collision|BreakHitResult _array_element))) "/Game/Characters/Towers/BP_BaseTower.BP_BaseTower_C")))
                        (LocalVariables|SetProjectileDirection (Math|Vector|GetUnitDirection(Vector) (LocalVariables|GetFirePointWorldPosition) (.ImpactPoint (Collision|BreakHitResult _array_element))))
                        (goto _label Break)
                        (else
                          _)))))
                (LocalVariables|SetProjectileDirection (LocalVariables|GetCameraWorldForwardVector))
                (goto _label Break)))
            (:then_2
              ;[1 1 1] Setup projectile movement parameters.
              (Utilities|Struct|SetmembersinMTD_ProjectileMovementParameters (.MovementParameters (Utilities|Struct|BreakMTD_ProjectileParameters (LocalVariables|GetProjectileParameters))) (Utilities|Struct|BreakMTD_EquipmentRangedWeaponStats (Variables|/Script/mtd.MTD_RangedWeaponInstance|GetRangedWeaponStats (LocalVariables|GetRangedWeaponInstance))) (Utilities|Struct|BreakMTD_EquipmentRangedWeaponStats (Variables|/Script/mtd.MTD_RangedWeaponInstance|GetRangedWeaponStats (LocalVariables|GetRangedWeaponInstance))) 0.0 (LocalVariables|GetProjectileDirection)))
            (:then_3
              ;[1 1 1] Setup projectile parameters.
              (bind _structout (Utilities|Struct|SetmembersinMTD_ProjectileParameters (LocalVariables|GetProjectileParameters) "(Name=\"NoCollision\")" (Class|MTDWeaponInstance|GetGameplayEffectSpecHandlestoGrantonHit (LocalVariables|GetRangedWeaponInstance))))
              (Utilities|Array|Add (.GameplayEffectsToGrantOnHit (Utilities|Struct|BreakMTD_ProjectileParameters _structout)) (CallFunction|CreateOutgoingRangedDamageSpecHandle))
              (Class|MTDProjectile|SetupProjectile (LocalVariables|GetProjectile) (LocalVariables|GetProjectileParameters)))))))))