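; Base enemy Blueprint that handles target selection, attack toggling, stat setup and death cleanup.
; Sight spheres track candidates, retargeting by nav path length on sight loss, and damage from players sets a target when none exists.
; Target changes and attack-trigger overlaps fire dispatchers; most-damage retargeting is left unwired.
; Level-scaled curve table stats initialize GAS through a SetByCaller effect, and death shrinks the mesh on timers before destroying the actor.
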(event OnComponentBeginOverlap(SightSphere)
  (params (OverlappedComponent :type Primitive%20Component%20Object%20Reference) (OtherActor :type Actor%20Object%20Reference) (OtherComp :type Primitive%20Component%20Object%20Reference) (OtherBodyIndex :type Integer) (bFromSweep :type Boolean) (SweepResult :type Hit%20Result%20Structure%20%28by%20ref%29))
  ;[1 1 1] Sight.
  (Utilities|Array|Add (Variables|MTD|Attack|GetDetectedTargets) OtherActor)
  (Utilities|IsValid (Variables|MTD|Attack|GetTarget)
    (:Is%20Not%20Valid
      (CallFunction|SetNewTarget OtherActor))))

(event OnComponentEndOverlap(LoseSightSphere)
  (params (OverlappedComponent :type Primitive%20Component%20Object%20Reference) (OtherActor :type Actor%20Object%20Reference) (OtherComp :type Primitive%20Component%20Object%20Reference) (OtherBodyIndex :type Integer))
  ;[1 1 1] Sight.
  (Utilities|Array|RemoveItem (Variables|MTD|Attack|GetDetectedTargets) OtherActor)
  (Utilities|IsValid (Variables|MTD|Attack|GetTarget)
    (:Is%20Valid
      (CallFunction|SetNewTarget (CallFunction|GetClosestTarget)))))

(event OnComponentBeginOverlap(AttackTrigger)
  (params (OverlappedComponent :type Primitive%20Component%20Object%20Reference) (OtherActor :type Actor%20Object%20Reference) (OtherComp :type Primitive%20Component%20Object%20Reference) (OtherBodyIndex :type Integer) (bFromSweep :type Boolean) (SweepResult :type Hit%20Result%20Structure%20%28by%20ref%29))
  ;[1 1 1] Attack.
  (bind _returnvalue (Utilities|Array|Add (Variables|MTD|Attack|GetAttackTargets) OtherActor))
  (if (== _returnvalue 0)
    (Default|CallToggleAttackingEventDispatcher)))

(event OnComponentEndOverlap(AttackTrigger)
  (params (OverlappedComponent :type Primitive%20Component%20Object%20Reference) (OtherActor :type Actor%20Object%20Reference) (OtherComp :type Primitive%20Component%20Object%20Reference) (OtherBodyIndex :type Integer))
  (bind _attacktargets (Variables|MTD|Attack|GetAttackTargets))
  ;[1 1 1] Attack.
  (Utilities|Array|RemoveItem _attacktargets OtherActor)
  (if (Utilities|Array|IsEmpty _attacktargets)
    (Default|CallToggleAttackingEventDispatcher)))

(event Custom|ScaleDown
  (bind _mesh (Variables|Character|GetMesh))
  ;[1 1 1] Death.
  ;;[1 1 1] Perform a single scale down step. The code will be called several times per second.
  (Transformation|SetRelativeScale3D _mesh (- (Variables|/Script/Engine.SceneComponent|GetRelativeScale3D _mesh) (* (/ (/ 1.0 (Variables|MTD|Death|GetScaleDownTickrate)) (Variables|MTD|Death|GetSecondsToCompleteScaleDown)) (Variables|MTD|Death|GetInitialScale)))))

(event Custom|OnDestroy
  ;[1 1 1] Death.
  ;;[1 1 1] Setup scale down and destroy timers.
  (Variables|MTD|Death|SetInitialScale (Variables|/Script/Engine.SceneComponent|GetRelativeScale3D (Variables|Character|GetMesh)))
  (bind _returnvalue (Utilities|Time|SetTimerbyEvent (delegate Custom|ScaleDown) (/ 1.0 (Variables|MTD|Death|GetScaleDownTickrate)) true))
  (Utilities|Time|SetTimerbyEvent (delegate Custom|FinishScalingDown) (Variables|MTD|Death|GetSecondsToCompleteScaleDown))
  ;;[1 1 1] Deactivate sight spheres.
  (Components|Activation|Deactivate (Variables|Default|GetSightSphere))
  (Components|Activation|Deactivate (Variables|Default|GetLoseSightSphere)))

(event Custom|FinishScalingDown
  ;[1 1 1] Death.
  ;;[1 1 1] Destroy actor.
  (Utilities|Time|ClearandInvalidateTimerbyHandle (stale Custom|OnDestroy _returnvalue))
  (Actor|DestroyActor))

(event EventOnDeathFinished
  (params (OwningActor :type Actor%20Object%20Reference))
  ;[1 1 1] Death.
  ;;[1 1 1] Override death event. Scale down before destroying the actor.
  (Utilities|Time|SetTimerbyEvent (EventDispatchers|CreateEvent :!event Custom|OnDestroy) (Variables|MTD|Death|GetSecondsToStartScalingDown)))

(event EventOnGameTerminated
  (params (GameResult :type EMTD_GameResult%20Enum :default "Lose"))
  (Class|Pawn|DetachfromControllerPendingDestroy))

(event EventOnDeathStarted
  (params (OwningActor :type Actor%20Object%20Reference))
  ;[1 1 1] Death.
  (|CallParentFunction OwningActor))

(event EventBeginPlay
  (|CallParentFunction)
  ;[1 1 1] Listen for health changed in order to change target.
  (EventDispatchers|AssignOnHealthChangedDelegate (Variables|Default|GetHealthComponent) (EventDispatchers|CreateEvent :!event OnHealthChanged))
  (CallFunction|InitializeAttributes))

(event EventTick
  (params (DeltaSeconds :type Float%20%28single-precision%29))
  (|CallParentFunction DeltaSeconds))

(fn ConstructionScript
  (|CallParentFunction))

(fn SetNewTarget
  (params (NewTarget :type Actor%20Object%20Reference))
  (bind _returnvalue (Actor|GetComponentbyClass NewTarget "/Script/mtd.MTD_HealthComponent"))
  (if (!= NewTarget (Variables|MTD|Attack|GetTarget))
    (LocalVariables|SetOldTarget (Variables|MTD|Attack|GetTarget))
    (Variables|MTD|Attack|SetTarget NewTarget)
    (Utilities|FlowControl|Sequence
      (:then_0
        ;[1 1 1] Don't listen for old attack target death anymore.
        (Utilities|IsValid (LocalVariables|GetOldTarget)
          (:Is%20Valid
            (Utilities|IsValid (Actor|GetComponentbyClass (LocalVariables|GetOldTarget) "/Script/mtd.MTD_HealthComponent")
              (:Is%20Valid
                (EventDispatchers|UnbindEventfromOnDeathStarted (Actor|GetComponentbyClass (LocalVariables|GetOldTarget) "/Script/mtd.MTD_HealthComponent") (EventDispatchers|CreateEvent :!event OnTargetDied)))))))
      (:then_1
        ;[1 1 1] Listen for new attack target death.
        (Utilities|IsValid NewTarget
          (:Is%20Valid
            (Utilities|IsValid _returnvalue
              (:Is%20Valid
                (EventDispatchers|BindEventtoOnDeathStarted _returnvalue (EventDispatchers|CreateEvent :!event OnTargetDied)))))))
      (:then_2
        ;[1 1 1] Broadcast old and new attack targets.
        (Default|CallNewTargetEventDispatcher (LocalVariables|GetOldTarget) NewTarget)))))

(fn OnTargetDied
  (params (OwningActor :type Actor%20Object%20Reference))
  ;[1 1 1] Invalidate.
  (Variables|MTD|Attack|SetTarget 0))

(fn CanbeSeen
  (params (Target :type Actor%20Object%20Reference))
  (bind _returnvalue (Transformation|GetActorLocation))
  (bind _outhit (Collision|LineTraceByChannel _returnvalue (+ _returnvalue (* (Math|Vector|Normalize (- (Transformation|GetActorLocation Target) (Transformation|GetActorLocation))) (Components|Sphere|GetScaledSphereRadius (Variables|Default|GetLoseSightSphere)))) "TraceTypeQuery3" false 0 "None"))
  (return (== Target (.HitActor (Collision|BreakHitResult _outhit)))))

(fn OnHealthChanged
  (params (HealthComponent :type MTD%20Health%20Component%20Object%20Reference) (OldValue :type Float%20%28single-precision%29) (NewValue :type Float%20%28single-precision%29) (Instigator :type Actor%20Object%20Reference))
  (Development|PrintString (Utilities|String|Append "Health: " (Utilities|String|ToString(Float) NewValue)))
  (Utilities|IsValid Instigator
    (:Is%20Valid
      (bind _asbp_mtd_player_state (Utilities|Casting|CastToBP_MtdPlayerState Instigator))
      (LocalVariables|SetInstigatorPawn (PlayerState|GetPawn _asbp_mtd_player_state))
      (bind _output_get (LocalVariables|SetDamage (- OldValue NewValue)))
      (if (> _output_get 0.0)
        (Utilities|FlowControl|Sequence
          (:then_2
            ;[1 1 1] Immediately target the damage instigator if there's no one to target.
            (Utilities|IsValid (Variables|MTD|Attack|GetTarget)
              (:Is%20Not%20Valid
                (CallFunction|SetNewTarget (LocalVariables|GetInstigatorPawn))))))))))

(fn InitializeAttributes
  (bind _returnvalue (Class|MTDBaseCharacter|GetMtdAbilitySystemComponent))
  (bind _level (LocalVariables|GetLevel))
  (bind _basestats (Variables|MTD|GetBaseStats))
  (bind (_health _damage _speed _mana) (Utilities|Struct|BreakF_EnemyStats _basestats))
  (bind _asmtd_game_mode_base (Utilities|Casting|CastToMTD_GameModeBase (Game|GetGameMode)))
  (bind _output_get (LocalVariables|SetGameModeBase _asmtd_game_mode_base))
  (Utilities|IsValid (Variables|/Script/mtd.MTD_GameModeBase|GetLevelDefinition _output_get)
    (:Is%20Valid
      (bind _output_get_2 (LocalVariables|SetLevelDefinition (Variables|/Script/mtd.MTD_GameModeBase|GetLevelDefinition _output_get)))
      (Utilities|IsValid (Variables|/Script/mtd.MTD_LevelDefinition|GetEntitiesAttributeTable _output_get_2)
        (:Is%20Valid
          (LocalVariables|SetInitGeSpecHandle (GameplayEffects|MakeOutgoingSpec _returnvalue "/Game/GameplayEffects/GE_EnemyStats.GE_EnemyStats_C" 1.0 (GameplayEffects|MakeEffectContext _returnvalue)))
          (bind _outxy (DataTable|EvaluateCurveTableRow (Variables|/Script/mtd.MTD_LevelDefinition|GetEntitiesAttributeTable _output_get_2) "HealthScale" _level)
            (:RowFound
              (bind _outxy_2 (DataTable|EvaluateCurveTableRow (Variables|/Script/mtd.MTD_LevelDefinition|GetEntitiesAttributeTable _output_get_2) "DamageScale" _level)
                (:RowFound
                  (bind _outxy_3 (DataTable|EvaluateCurveTableRow (Variables|/Script/mtd.MTD_LevelDefinition|GetEntitiesAttributeTable _output_get_2) "SpeedScale" _level)
                    (:RowFound
                      (bind _structout (Utilities|Struct|SetmembersinF_EnemyStats (LocalVariables|GetFinalStats) (* _outxy _health) (* _outxy_2 _damage) (* _outxy_3 _speed) _mana))
                      ;[1 1 1] This supposes that the enemy will never change its stats after initialization.
                      (bind _returnvalue_2 (Ability|GameplayEffect|AssignTagSetbyCallerMagnitude (LocalVariables|GetInitGeSpecHandle) "(TagName=\"SetByCaller.Health\")" (.Health (Utilities|Struct|BreakF_EnemyStats _structout))))
                      (bind _returnvalue_3 (Ability|GameplayEffect|AssignTagSetbyCallerMagnitude _returnvalue_2 "(TagName=\"SetByCaller.MaxHealth\")" (.Health (Utilities|Struct|BreakF_EnemyStats _structout))))
                      (bind _returnvalue_4 (Ability|GameplayEffect|AssignTagSetbyCallerMagnitude _returnvalue_3 "(TagName=\"SetByCaller.Damage.Base\")" (.Damage (Utilities|Struct|BreakF_EnemyStats _structout))))
                      (bind _returnvalue_5 (Ability|GameplayEffect|AssignTagSetbyCallerMagnitude _returnvalue_4 "(TagName=\"SetByCaller.MaxMana\")" (.Mana (Utilities|Struct|BreakF_EnemyStats _structout))))
                      (GameplayEffects|ApplyGameplayEffectSpecToSelf (Class|MTDBaseCharacter|GetMtdAbilitySystemComponent) _returnvalue_5)
                      (return))
                    (:RowNotFound
                      _)))
                (:RowNotFound
                  _)))
            (:RowNotFound
              _))
          (Development|PrintString (Utilities|String|Append "Couldn't find a value in " (Utilities|GetDisplayName (LocalVariables|GetLevelDefinition)) "'s Entities Attribute Table")))))))

(fn OnTryChangeTarget
  (bind _output_get (LocalVariables|SetMostDealing (CallFunction|FindMostDealingInstigator)))
  (Utilities|IsValid _output_get
    (:Is%20Valid
      ;[1 1 1] Set new attack target if the most dealing instigator is not the current attack target.
      (if (!= (LocalVariables|GetMostDealing) (Variables|MTD|Attack|GetTarget))
        (CallFunction|SetNewTarget)))))

(fn FindMostDealingInstigator
  (bind _lastdamageinstigators (Variables|MTD|Targetting|GetLastDamageInstigators))
  (if (Utilities|Map|IsNotEmpty _lastdamageinstigators)
    (bind _values (Utilities|Map|Values _lastdamageinstigators))
    (LocalVariables|SetMostDamage (Utilities|Array|Get(acopy) _values))
    (for (_array_element _array_index) _values
      (if (> _array_element (LocalVariables|GetMostDamage))
        (LocalVariables|SetMostDamage _array_element)
        (LocalVariables|SetMostDamageIndex _array_index)))
    (bind _keys (Utilities|Map|Keys (Variables|MTD|Targetting|GetLastDamageInstigators)))
    (return (Utilities|Array|Get(acopy) _keys (LocalVariables|GetMostDamageIndex)))))

(fn GetClosestTarget
  ;[1 1 1] Cache.
  (LocalVariables|SetOurLocation (Pawn|GetNavAgentLocation))
  (LocalVariables|SetShortestDistance 0.0)
  (LocalVariables|SetFilterClass (Variables|/Script/AIModule.AIController|GetDefaultNavigationFilterClass (AI|GetAIController (Pawn|GetController))))
  (for _array_element (Variables|MTD|Attack|GetDetectedTargets)
    (if (Utilities|Select :Index (.ReturnValue (Class|NavigationSystemV1|GetPathLength (LocalVariables|GetOurLocation) (Transformation|GetActorLocation _array_element) 0 (LocalVariables|GetFilterClass))) :Invalid false :Error false :Fail false :Success true)
      (if (or (Utilities|IsValid (LocalVariables|GetClosestTarget)) (> (LocalVariables|GetShortestDistance) (.PathLength (Class|NavigationSystemV1|GetPathLength (LocalVariables|GetOurLocation) (Transformation|GetActorLocation _array_element) 0 (LocalVariables|GetFilterClass)))))
        (LocalVariables|SetClosestTarget _array_element)
        (LocalVariables|SetShortestDistance (.PathLength (Class|NavigationSystemV1|GetPathLength (LocalVariables|GetOurLocation) (Transformation|GetActorLocation _array_element) 0 (LocalVariables|GetFilterClass)))))))
  (return (LocalVariables|GetClosestTarget)))