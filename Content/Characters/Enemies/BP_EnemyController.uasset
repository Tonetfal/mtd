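; AI controller for BP_BaseEnemy pawns that runs the enemy's default behavior tree and registers a sight stimuli source on possession.
; It follows the enemy's new-target dispatcher, writing the target to the Blackboard and moving death listeners between targets.
; Pawn death unregisters sight and stops the behavior tree.
; The target-death handler stops logic only on a dead actor that casts to BP_BaseEnemy.
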(event EventUnPossess
  (params (UnpossessedPawn :type Pawn%20Object%20Reference))
  (bind _returnvalue (Actor|GetComponentbyClass UnpossessedPawn "/Script/mtd.MTD_HealthComponent"))
  ;[1 1 1] Don't listen for owner death anymore.
  (Utilities|FlowControl|Sequence
    (:then_0
      (Utilities|IsValid UnpossessedPawn
        (:Is%20Valid
          (Utilities|IsValid _returnvalue
            (:Is%20Valid
              (EventDispatchers|UnbindEventfromOnDeathStarted _returnvalue (EventDispatchers|CreateEvent :!event OnPawnDied)))))))))

(event EventPossess
  (params (PossessedPawn :type Pawn%20Object%20Reference))
  (Utilities|IsValid PossessedPawn
    (:Is%20Valid
      (bind _asbp_base_enemy (Utilities|Casting|CastToBP_BaseEnemy PossessedPawn)
        (:then
          (Utilities|FlowControl|Sequence
            (:then_0
              ;[1 1 1] Listen for new attack targets.
              (EventDispatchers|BindEventtoNewTargetEventDispatcher _asbp_base_enemy (EventDispatchers|CreateEvent :!event OnNewAttackTarget)))
            (:then_1
              ;[1 1 1] Listen for attack owner death.
              (Utilities|IsValid (Variables|/Script/mtd.MTD_BaseCharacter|GetHealthComponent _asbp_base_enemy)
                (:Is%20Valid
                  (EventDispatchers|AssignOnDeathStarted (Variables|/Script/mtd.MTD_BaseCharacter|GetHealthComponent _asbp_base_enemy) (EventDispatchers|CreateEvent :!event OnPawnDied)))))
            (:then_2
              ;[1 1 1] Run behavior tree.
              (Utilities|IsValid (Variables|/Game/Characters/Enemies/BP_BaseEnemy.BP_BaseEnemy_C|GetBehaviorTree _asbp_base_enemy)
                (:Is%20Valid
                  (Utilities|IsValid (Variables|/Script/AIModule.BehaviorTreeComponent|GetDefaultBehaviorTreeAsset (Variables|/Game/Characters/Enemies/BP_BaseEnemy.BP_BaseEnemy_C|GetBehaviorTree _asbp_base_enemy))
                    (:Is%20Valid
                      (AI|RunBehaviorTree (Variables|/Script/AIModule.BehaviorTreeComponent|GetDefaultBehaviorTreeAsset (Variables|/Game/Characters/Enemies/BP_BaseEnemy.BP_BaseEnemy_C|GetBehaviorTree _asbp_base_enemy))))))))
            (:then_3
              ;[1 1 1] Register for sight sense.
              (Class|AIPerceptionStimuliSourceComponent|RegisterforSense (Variables|Default|GetAI%20Perception%20Stimuli%20Source) "/Script/AIModule.AISense_Sight"))))
        (:CastFailed
          (Development|PrintString (Utilities|String|Append (Utilities|GetDisplayName PossessedPawn) " is not of type BP_BaseEnemy")))))))

(fn ConstructionScript)

(fn OnAttackTargetDied
  (params (Owning%20Actor :type Actor%20Object%20Reference))
  (bind _asbp_base_enemy (Utilities|Casting|CastToBP_BaseEnemy Owning%20Actor))
  (Utilities|IsValid (Variables|/Game/Characters/Enemies/BP_BaseEnemy.BP_BaseEnemy_C|GetBehaviorTree _asbp_base_enemy)
    (:Is%20Valid
      (AI|Logic|StopLogic (Variables|/Game/Characters/Enemies/BP_BaseEnemy.BP_BaseEnemy_C|GetBehaviorTree _asbp_base_enemy) "Character died"))))

(fn OnNewAttackTarget
  (params (OldTarget :type Actor%20Object%20Reference) (NewTarget :type Actor%20Object%20Reference))
  (bind _returnvalue (Actor|GetComponentbyClass NewTarget "/Script/mtd.MTD_HealthComponent"))
  (bind _returnvalue_2 (Actor|GetComponentbyClass OldTarget "/Script/mtd.MTD_HealthComponent"))
  (Utilities|FlowControl|Sequence
    (:then_0
      (Utilities|IsValid OldTarget
        (:Is%20Valid
          (Utilities|IsValid _returnvalue_2
            (:Is%20Valid
              (EventDispatchers|UnbindEventfromOnDeathStarted _returnvalue_2 (EventDispatchers|CreateEvent :!event OnAttackTargetDied)))))))
    (:then_1
      (Utilities|IsValid NewTarget
        (:Is%20Valid
          (Utilities|IsValid _returnvalue
            (:Is%20Valid
              (EventDispatchers|BindEventtoOnDeathStarted _returnvalue (EventDispatchers|CreateEvent :!event OnAttackTargetDied)))))))
    (:then_2
      (AI|Components|Blackboard|SetValueasObject (Variables|Default|GetBlackboard) (Variables|Default|GetBlackboardAttackTargetKeyName) NewTarget))))

(fn OnPawnDied
  (params (OwningActor :type Actor%20Object%20Reference))
  (Class|AIPerceptionStimuliSourceComponent|UnregisterfromSense (Variables|Default|GetAI%20Perception%20Stimuli%20Source) "/Script/AIModule.AISense_Sight")
  (AI|Logic|StopLogic (Variables|Default|GetBehaviorTree) "Owner has died"))