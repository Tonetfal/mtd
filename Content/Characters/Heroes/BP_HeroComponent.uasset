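; BP_HeroComponent is a hero character component that decides whether the hero can look and move.
; It caches the Mtd ability system component on BeginPlay.
; The CanLook and CanMove checks read that component's owned gameplay tags and deny both while the exact Gameplay.Effects.BuildSystem.Building tag is present, locking camera and movement during building.
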(event EventBeginPlay
  (Variables|Default|SetMtdAbilitySystemComponent (Class|MTDHeroComponent|GetMtdAbilitySystemComponent)))

(fn K2CanLook
  (bind _mtdabilitysystemcomponent (Variables|Default|GetMtdAbilitySystemComponent))
  (Utilities|IsValid _mtdabilitysystemcomponent
    (:Is%20Valid
      (return (not (GameplayTags|HasTag (GameplayTags|GetOwnedGameplayTags _mtdabilitysystemcomponent :!class /Script/GameplayTags.GameplayTagAssetInterface) "(TagName=\"Gameplay.Effects.BuildSystem.Building\")" true))))))

(fn K2CanMove
  (bind _mtdabilitysystemcomponent (Variables|Default|GetMtdAbilitySystemComponent))
  (Utilities|IsValid _mtdabilitysystemcomponent
    (:Is%20Valid
      (return (not (GameplayTags|HasTag (GameplayTags|GetOwnedGameplayTags _mtdabilitysystemcomponent :!class /Script/GameplayTags.GameplayTagAssetInterface) "(TagName=\"Gameplay.Effects.BuildSystem.Building\")" true))))))