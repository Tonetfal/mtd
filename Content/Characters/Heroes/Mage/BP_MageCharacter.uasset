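; Mage hero character Blueprint that currently adds only debug readouts for enemy spawning on top of its parent class.
; After parent BeginPlay, it finds the BP_EnemySpawner actor and prints the total spawn counts for the two test enemy classes.
; An L debug key repeats the same lookup and printout, and the construction script only calls the parent.
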(event EventBeginPlay
  (|CallParentFunction)
  (bind _returnvalue (Actor|GetActorOfClass "/Game/Gameplay/Spawners/BP_EnemySpawner.BP_EnemySpawner_C"))
  (Development|PrintString (Utilities|String|ToString(Integer) (Class|MTDCharacterSpawner|GetTotalCharactersOfClasstoSpawn _returnvalue "/Game/Characters/Enemies/Test/BP_TestEnemy.BP_TestEnemy_C")))
  (Development|PrintString (Utilities|String|ToString(Integer) (Class|MTDCharacterSpawner|GetTotalCharactersOfClasstoSpawn _returnvalue "/Game/Characters/Enemies/Test2/BP_TestEnemy2.BP_TestEnemy2_C"))))

(event Input|KeyboardEvents|DebugKeyL
  (params (Key :type Key%20Structure :default "None") (ActionValue :type Input%20Action%20Value%20Structure))
  (:Pressed
    (bind _returnvalue (Actor|GetActorOfClass "/Game/Gameplay/Spawners/BP_EnemySpawner.BP_EnemySpawner_C"))
    (Development|PrintString (Utilities|String|ToString(Integer) (Class|MTDCharacterSpawner|GetTotalCharactersOfClasstoSpawn _returnvalue "/Game/Characters/Enemies/Test/BP_TestEnemy.BP_TestEnemy_C")))
    (Development|PrintString (Utilities|String|ToString(Integer) (Class|MTDCharacterSpawner|GetTotalCharactersOfClasstoSpawn _returnvalue "/Game/Characters/Enemies/Test2/BP_TestEnemy2.BP_TestEnemy2_C")))))

(fn ConstructionScript
  (|CallParentFunction))