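; Base Blueprint for hero player characters, handling input setup, starting attributes and input shutdown on death or game end.
; BeginPlay registers with the GameFrameworkComponentManager, adds the Enhanced Input mapping context and initializes attributes.
; Health and Mana come from PlayerData's curve table by Level, applied via GE_PlayerStats SetByCaller magnitudes, though starting Mana is hard-coded.
; Helpers expose the player controller and consume turn input, whose setter is unconnected.
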(event Input|EnhancedActionEvents|EnhancedInputActionIA_Look_Mouse
  (params (ActionValue :type Vector%202D%20Structure) (ElapsedSeconds :type Float%20%28double-precision%29) (TriggeredSeconds :type Float%20%28double-precision%29) (InputAction :type Input%20Action%20Object%20Reference :default "/Game/Input/Actions/IA_Look_Mouse.IA_Look_Mouse")))

(event EventBeginPlay
  (Class|GameFrameworkComponentManager|AddReceiver (Subsystems|GetGameFrameworkComponentManager))
  (|CallParentFunction)
  (Utilities|FlowControl|Sequence
    (:then_0
      ;[1 1 1] Initialize input.
      (bind _asplayer_controller (Utilities|Casting|CastToPlayerController (Pawn|GetController)))
      (Input|AddMappingContext (PlayerController|LocalPlayerSubsystems|GetEnhancedInputLocalPlayerSubsystem _asplayer_controller) (Variables|MTD|Input|GetInputMappingContext) 0 "(bIgnoreAllPressedKeysUntilRelease=True,bForceImmediately=False)"))
    (:then_1
      ;[1 1 1] Initialize attributes.
      (CallFunction|InitializeAttributes))))

(event EventOnDeathStarted
  (params (OwningActor :type Actor%20Object%20Reference))
  (bind _returnvalue (Pawn|GetController))
  (|CallParentFunction 0)
  (Utilities|IsValid _returnvalue
    (:Is%20Valid
      (bind _asplayer_controller (Utilities|Casting|CastToPlayerController _returnvalue))
      (Input|DisableInput _asplayer_controller))))

(event EventOnGameTerminated
  (params (GameResult :type E_GameResult%20Enum :default "NewEnumerator0"))
  (bind _returnvalue (Pawn|GetController))
  (switch Utilities|FlowControl|Switch|SwitchonE_GameResult GameResult
    (:NewEnumerator0
      _)
    (:NewEnumerator1
      _))
  (Utilities|IsValid _returnvalue
    (:Is%20Valid
      (bind _asplayer_controller (Utilities|Casting|CastToPlayerController _returnvalue))
      (Input|DisableInput _asplayer_controller)
      (Input|SetIgnoreLookInput _asplayer_controller false))))

(event EventOnReset
  (Variables|/Script/Engine.CharacterMovementComponent|SetbUseControllerDesiredRotation (Variables|Character|GetCharacterMovement) true))

(fn ConstructionScript
  (|CallParentFunction))

(fn ConsumeTurnRatio
  (LocalVariables|SetTurnRatioTmp (Variables|MTD|Animation|GetTurnRatio))
  (LocalVariables|SetbIsTurningTmp (Variables|MTD|Animation|GetbIsTurning))
  (Variables|MTD|Animation|SetbIsTurning false)
  (Variables|MTD|Animation|SetTurnRatio 0.0)
  (return (LocalVariables|GetbIsTurningTmp) (LocalVariables|GetTurnRatioTmp)))

(fn DisableControllerInput
  (bind _returnvalue (Pawn|GetController))
  (bind _charactermovement (Variables|Character|GetCharacterMovement))
  (Utilities|IsValid _returnvalue
    (:Is%20Valid
      (Input|SetIgnoreMoveInput _returnvalue false)
      (Utilities|IsValid _charactermovement
        (:Is%20Valid
          (Variables|/Script/Engine.CharacterMovementComponent|SetbUseControllerDesiredRotation _charactermovement false))))))

(fn InitializeAttributes
  (bind _returnvalue (Class|MTDBaseCharacter|GetMtdAbilitySystemComponent))
  (bind _level (Variables|MTD|GetLevel))
  (bind _pawnextentioncomponent (Variables|Default|GetPawnExtentionComponent))
  (bind _playerdata (Variables|/Script/mtd.MTD_PawnExtensionComponent|GetPlayerData _pawnextentioncomponent))
  (bind _attributetable (Variables|/Script/mtd.MTD_PlayerData|GetAttributeTable _playerdata))
  (Utilities|IsValid _playerdata
    (:Is%20Valid
      (Utilities|IsValid _attributetable
        (:Is%20Valid
          (LocalVariables|SetInitGeSpecHandle (GameplayEffects|MakeOutgoingSpec _returnvalue "/Game/GameplayEffects/GE_PlayerStats.GE_PlayerStats_C" 1.0 (GameplayEffects|MakeEffectContext _returnvalue)))
          (bind _outxy (DataTable|EvaluateCurveTableRow _attributetable "Health" _level)
            (:RowFound
              (LocalVariables|SetHealth _outxy)
              (bind _outxy_2 (DataTable|EvaluateCurveTableRow _attributetable "Mana" _level)
                (:RowFound
                  (LocalVariables|SetMana _outxy_2)
                  (bind _returnvalue_2 (Ability|GameplayEffect|AssignTagSetbyCallerMagnitude (LocalVariables|GetInitGeSpecHandle) "(TagName=\"SetByCaller.Health\")" (LocalVariables|GetHealth)))
                  (bind _returnvalue_3 (Ability|GameplayEffect|AssignTagSetbyCallerMagnitude _returnvalue_2 "(TagName=\"SetByCaller.MaxHealth\")" (LocalVariables|GetHealth)))
                  (bind _returnvalue_4 (Ability|GameplayEffect|AssignTagSetbyCallerMagnitude _returnvalue_3 "(TagName=\"SetByCaller.Mana\")" 1e+01))
                  (bind _returnvalue_5 (Ability|GameplayEffect|AssignTagSetbyCallerMagnitude _returnvalue_4 "(TagName=\"SetByCaller.MaxMana\")" (LocalVariables|GetMana)))
                  (GameplayEffects|ApplyGameplayEffectSpecToSelf (Class|MTDBaseCharacter|GetMtdAbilitySystemComponent) _returnvalue_5))))
            (:RowNotFound
              (Development|PrintString (Utilities|String|Append "Player Default Attribute on owner [" (Utilities|GetDisplayName self) "] misses a value. The searched column is [" (Utilities|String|ToString(Float) (Variables|MTD|GetLevel)) "]")))))))))

(fn GetMtdPlayerController
  (bind _returnvalue (Pawn|GetController))
  (Utilities|IsValid _returnvalue
    (:Is%20Valid
      (bind _asmtd_player_controller (Utilities|Casting|CastToMTD_PlayerController _returnvalue)
        (:then
          _)
        (:CastFailed
          _))
      (return _asmtd_player_controller))))