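; Base character Blueprint that equips a default weapon on spawn and handles melee hit detection for the Gameplay Ability System.
; BeginPlay maps hitbox nicknames to HitboxData spheres, which events activate or remove by name.
; While any are active, Tick sphere-traces them relative to actor facing, sending itself a gameplay event once per new target until reset.
; A helper returns the signed angle between facing and velocity.
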(event EventBeginPlay
  (CallFunction|ContructHitboxMap)
  (CallFunction|EquipItemsonSpawn))

(event EventTick
  (params (DeltaSeconds :type Float%20%28single-precision%29))
  (if (Variables|MTD|Attack|GetIsMeleeInProgress)
    (CallFunction|EventPerformHitboxTrace)))

(event Custom|EventPerformHitboxTrace
  (bind _meleehittargets (Variables|MTD|Attack|GetMeleeHitTargets))
  ;[1 1 1] Ignore if there are no active hitboxes.
  (if (> (Utilities|Array|Length (Variables|MTD|Attack|GetActiveHitboxes)) 0)
    ;[1 1 1] Check if hitboxes are hitting something.
    (for _array_element (Variables|MTD|Attack|GetActiveHitboxes)
      (bind (_outhits _returnvalue) (Collision|MultiSphereTraceForObjects (+ (Transformation|GetActorLocation) (Math|Vector|RotateVector (.Offset (Utilities|Struct|BreakMeleeHitSphereDefinition _array_element)) (Math|Conversions|RotationFromXVector (Transformation|GetActorForwardVector)))) (+ (Transformation|GetActorLocation) (Math|Vector|RotateVector (.Offset (Utilities|Struct|BreakMeleeHitSphereDefinition _array_element)) (Math|Conversions|RotationFromXVector (Transformation|GetActorForwardVector)))) (.Radius (Utilities|Struct|BreakMeleeHitSphereDefinition _array_element)) (Variables|MTD|Attack|GetTargetCollisionProfilesToHit) false 0 (select (Variables|MTD|Attack|GetDebugMelee) "ForDuration" "None") true "(R=1.000000,G=0.000000,B=0.000000,A=1.000000)" "(R=0.000000,G=1.000000,B=0.000000,A=1.000000)" 0.0))
      (if _returnvalue
        (for _array_element_2 _outhits
          ;[1 1 1] Check if actor has been already hit.
          (if (not (Utilities|Array|ContainsItem _meleehittargets (.HitActor (Collision|BreakHitResult _array_element_2))))
            (Utilities|Array|AddUnique _meleehittargets (.HitActor (Collision|BreakHitResult _array_element_2)))
            ;[1 1 1] Apply damage gameplay effect to the hitting target.
            (Ability|SendGameplayEventtoActor self (Variables|Default|GetGameplayTagToFireOnHit) (Utilities|Struct|MakeGameplayEventData "(TagName=\"\")" (Variables|Default|GetPlayerState) (.HitActor (Collision|BreakHitResult _array_element_2)) 0 0 (GameplayEffects|MakeEffectContext (Class|MTDBaseCharacter|GetMtdAbilitySystemComponent)) "(GameplayTags=)" "(GameplayTags=)" 1.0 (Ability|TargetData|AbilityTargetDatafromHitResult _array_element_2)))))))))

(event EventAddMeleeHitboxes
  (params (MeleeHitboxes :type Array%20of%20Names))
  ;[1 1 1] Adds hitboxes with given nicknames.
  (for _array_element MeleeHitboxes
    (if (.ReturnValue (Utilities|Map|Find (Variables|MTD|Attack|GetHitboxMap) _array_element))
      (Utilities|Array|AddUnique (Variables|MTD|Attack|GetActiveHitboxes) (Utilities|Struct|BreakF_ActiveHitboxEntry (.Value (Utilities|Map|Find (Variables|MTD|Attack|GetHitboxMap) _array_element))))))
  (Variables|MTD|Attack|SetIsMeleeInProgress (> (Utilities|Array|Length (Variables|MTD|Attack|GetActiveHitboxes)) 0)))

(event EventDisableMeleeHitboxes
  ;[1 1 1] Forcibly kills all active melee hitboxes, and empties the list.
  (Variables|MTD|Attack|SetIsMeleeInProgress false)
  (Utilities|Array|Clear (Variables|MTD|Attack|GetActiveHitboxes))
  (CallFunction|ResetMeleeHitboxes))

(event EventResetMeleeHitboxes
  ;[1 1 1] Resets the active hitboxes so that hit detection can be performed on target again.
  (Utilities|Array|Clear (Variables|MTD|Attack|GetMeleeHitTargets)))

(event EventRemoveMeleeHitboxes
  (params (MeleeHitboxes :type Array%20of%20Names))
  ;[1 1 1] Removes hitboxes with given nicknames.
  (for _array_element MeleeHitboxes
    (if (.ReturnValue (Utilities|Map|Find (Variables|MTD|Attack|GetHitboxMap) _array_element))
      (Utilities|Array|RemoveItem (Variables|MTD|Attack|GetActiveHitboxes) (Utilities|Struct|BreakF_ActiveHitboxEntry (.Value (Utilities|Map|Find (Variables|MTD|Attack|GetHitboxMap) _array_element))))))
  (bind _output_get (Variables|MTD|Attack|SetIsMeleeInProgress (> (Utilities|Array|Length (Variables|MTD|Attack|GetActiveHitboxes)) 0)))
  (if (not _output_get)
    (CallFunction|ResetMeleeHitboxes)))

(fn ConstructionScript)

(fn ContructHitboxMap
  (Utilities|Map|Clear (Variables|MTD|Attack|GetHitboxMap))
  (for _array_element (Variables|/Script/mtd.MeleeHitboxData|GetMeleeHitSpheres (Variables|MTD|Attack|GetHitboxData))
    (Utilities|Map|Add (Variables|MTD|Attack|GetHitboxMap) (.Nickname (Utilities|Struct|BreakMeleeHitSphereDefinition _array_element)) (Utilities|Struct|MakeF_ActiveHitboxEntry _array_element))))

(fn GetMovementDirectionAngle
  (bind _returnvalue (Transformation|GetVelocity))
  (bind _returnvalue_2 (Transformation|GetActorForwardVector))
  (bind _returnvalue_3 (Class|KismetMathLibrary|VectorNormalUnsafe _returnvalue))
  (bind _returnvalue_4 (Math|Vector|DotProduct _returnvalue_2 _returnvalue_3))
  (bind _returnvalue_5 (Math|Vector|CrossProduct _returnvalue_2 _returnvalue_3))
  (bind _returnvalue_6 (Class|KismetMathLibrary|DegAcos _returnvalue_4))
  (if (not (Math|Vector|VectorIsZero _returnvalue))
    (if (Math|Vector|VectorIsZero _returnvalue_5)
      (return _returnvalue_6)
      (else
        (return (* _returnvalue_6 (Math|Float|Sign(Float) (.Z (Class|KismetMathLibrary|BreakVector3f _returnvalue_5)))))))))

(fn EquipItemsonSpawn
  (bind _defaultweapondefinitionclass (Variables|Default|GetDefaultWeaponDefinitionClass))
  (if (Utilities|IsValidClass _defaultweapondefinitionclass)
    (Class|MTDEquipmentManagerComponent|EquipItem (Variables|Default|GetMTD_EquipmentManager) _defaultweapondefinitionclass)))