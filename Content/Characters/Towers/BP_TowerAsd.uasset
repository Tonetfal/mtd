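; Tower character Blueprint that sets up its combat stats on BeginPlay and detaches from its controller when the game terminates.
; It evaluates the TowerData curve table at the tower's Level for health, damage, range, vision angle, fire rate and projectile speed.
; Health goes through a SetByCaller GameplayEffect, while the other stats become base variables.
; Scaled vision range and half-angle are then pushed to BP_TowerController.
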(event EventOnGameTerminated
  (params (GameResult :type EMTD_GameResult%20Enum :default "Lose"))
  (Class|Pawn|DetachfromControllerPendingDestroy))

(event EventBeginPlay
  (CallFunction|InitializeAttributes))

(fn ConstructionScript)

(fn InitializeAttributes
  (bind _returnvalue (Pawn|GetController))
  (bind _returnvalue_2 (Class|MTDTowerAsd|GetMtdAbilitySystemComponent))
  (bind _towerdata (Variables|Default|GetTowerData))
  (bind _level (Variables|Default|GetLevel))
  (bind _attributetable (Variables|/Script/mtd.MTD_TowerData|GetAttributeTable _towerdata))
  (Utilities|IsValid _towerdata
    (:Is%20Valid
      (Utilities|IsValid _attributetable
        (:Is%20Valid
          (LocalVariables|SetInitGeSpecHandle (GameplayEffects|MakeOutgoingSpec _returnvalue_2 "/Game/GameplayEffects/GE_TowerStats.GE_TowerStats_C" 1.0 (GameplayEffects|MakeEffectContext _returnvalue_2)))
          ;[1 1 1] Retrieve table values.
          (bind _outxy (DataTable|EvaluateCurveTableRow _attributetable "Health" _level)
            (:RowFound
              (bind _outxy_2 (DataTable|EvaluateCurveTableRow _attributetable "Damage" _level)
                (:RowFound
                  (bind _outxy_3 (DataTable|EvaluateCurveTableRow _attributetable "Range" _level)
                    (:RowFound
                      (bind _outxy_4 (DataTable|EvaluateCurveTableRow _attributetable "VisionDegrees" _level)
                        (:RowFound
                          (bind _outxy_5 (DataTable|EvaluateCurveTableRow _attributetable "Firerate" _level)
                            (:RowFound
                              (bind _outxy_6 (DataTable|EvaluateCurveTableRow _attributetable "ProjectileSpeed" _level)
                                (:RowFound
                                  ;[1 1 1] Apply retrieved values.
                                  (Variables|Default|SetBaseProjectileSpeed _outxy_6)
                                  (Variables|Default|SetBaseFirerate _outxy_5)
                                  (Variables|Default|SetBaseVisionHalfDegrees (/ _outxy_4 2.0))
                                  (Variables|Default|SetBaseVisionRange _outxy_3)
                                  (Variables|Default|SetBaseDamage _outxy_2)
                                  (bind _returnvalue_3 (Ability|GameplayEffect|AssignTagSetbyCallerMagnitude (LocalVariables|GetInitGeSpecHandle) "(TagName=\"SetByCaller.Health\")" _outxy))
                                  (bind _returnvalue_4 (Ability|GameplayEffect|AssignTagSetbyCallerMagnitude _returnvalue_3 "(TagName=\"SetByCaller.MaxHealth\")" _outxy))
                                  (GameplayEffects|ApplyGameplayEffectSpecToSelf (Class|MTDTowerAsd|GetMtdAbilitySystemComponent) _returnvalue_4)
                                  (Utilities|IsValid _returnvalue
                                    (:Is%20Valid
                                      (bind _asbp_tower_controller (Utilities|Casting|CastToBP_TowerController _returnvalue))
                                      (Class|MTDTowerController|SetVisionRange _asbp_tower_controller (Class|MTDTowerAsd|GetScaledVisionRange))
                                      (Class|MTDTowerController|SetPeripheralVisionHalfAngleDegrees _asbp_tower_controller (Class|MTDTowerAsd|GetScaledVisionHalfDegrees)))))))))))))))
            (:RowNotFound
              (Development|PrintString (Utilities|String|Append "Tower Attribute on owner [" (Utilities|GetDisplayName self) "] misses a value. The searched column is [" (Utilities|String|ToString(Float) (Variables|Default|GetLevel)) "]")))))))))