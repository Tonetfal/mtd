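; BP_Tower is a tower Blueprint that drives a status bar widget showing the tower's health.
; On BeginPlay it registers as a Game Framework Component receiver for plugins, binds HealthComponent change delegates and starts the widget hidden and transparent.
; Health and max health changes refresh the bar's progress and text, but only while the widget is Visible.
; A visibility callback gates those updates and refreshes immediately when the bar becomes Visible.
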(event EventBeginPlay
  (bind _statusbar (Variables|Default|GetStatusBar))
  (bind _healthcomponent (Variables|Default|GetHealthComponent))
  (bind _returnvalue (UserInterface|GetWidget _statusbar))
  (Utilities|FlowControl|Sequence
    (:then_0
      (Utilities|FlowControl|Sequence
        (:then_0
          ;[1 1 1] Add plugins.
          (Class|GameFrameworkComponentManager|AddReceiver (Subsystems|GetGameFrameworkComponentManager)))
        (:then_1
          ;[1 1 1] Listen for health changes to update health bar.
          (EventDispatchers|BindEventtoOnHealthChangedDelegate _healthcomponent (EventDispatchers|CreateEvent :!event OnHealthChanged))
          (EventDispatchers|AssignOnMaxHealthChangedDelegate _healthcomponent (EventDispatchers|CreateEvent :!event OnMaxHealthChanged)))
        (:then_2
          ;[1 1 1] Initialize front-end.
          (Utilities|IsValid _returnvalue
            (:Is%20Valid
              (EventDispatchers|AssignOnVisibilityChanged _returnvalue (EventDispatchers|CreateEvent :!event OnHealthWidgetVisibilityChanged))
              (Widget|SetRenderOpacity _returnvalue 0.0)
              (Widget|SetVisibility _returnvalue "Hidden"))))))
    (:then_1
      (|CallParentFunction))))

(fn ConstructionScript)

(fn OnHealthChanged
  (params (HealthComponent :type MTD%20Health%20Component%20Object%20Reference) (OldValue :type Float%20%28single-precision%29) (NewValue :type Float%20%28single-precision%29) (Instigator :type Actor%20Object%20Reference))
  (CallFunction|UpdateHealthWidgetProgress))

(fn OnMaxHealthChanged
  (params (HealthComponent :type MTD%20Health%20Component%20Object%20Reference) (OldValue :type Float%20%28single-precision%29) (NewValue :type Float%20%28single-precision%29) (Instigator :type Actor%20Object%20Reference))
  (CallFunction|UpdateHealthWidgetProgress))

(fn UpdateHealthWidgetProgress
  (bind _statusbar (Variables|Default|GetStatusBar))
  (bind _healthcomponent (Variables|Default|GetHealthComponent))
  (bind _returnvalue (UserInterface|GetWidget _statusbar))
  (if (Variables|Default|GetbShouldHealthWidgetUpdate)
    (Utilities|IsValid _returnvalue
      (:Is%20Valid
        (bind _aswbp_tower_status_bar (Utilities|Casting|CastToWBP_TowerStatusBar _returnvalue))
        (Default|SetProgress (Variables|/Game/UI/Widgets/WBP_TowerStatusBar.WBP_TowerStatusBar_C|GetHealthBar _aswbp_tower_status_bar) (Class|MTDHealthComponent|GetHealthNormilized _healthcomponent))
        (Default|SetText (Variables|/Game/UI/Widgets/WBP_TowerStatusBar.WBP_TowerStatusBar_C|GetHealthBar _aswbp_tower_status_bar) (Class|MTDHealthComponent|GetHealth _healthcomponent) (Class|MTDHealthComponent|GetMaxHealth _healthcomponent))))))

(fn OnHealthWidgetVisibilityChanged
  (params (InVisibility :type ESlateVisibility%20Enum :default "Visible"))
  (switch Utilities|FlowControl|Switch|SwitchonESlateVisibility InVisibility
    (:Visible
      (Variables|Default|SetbShouldHealthWidgetUpdate true)
      (CallFunction|UpdateHealthWidgetProgress))
    (:Collapsed
      (Variables|Default|SetbShouldHealthWidgetUpdate false :!label _label))
    (:Hidden
      (goto _label))
    (:HitTestInvisible
      (goto _label))
    (:SelfHitTestInvisible
      (goto _label))))